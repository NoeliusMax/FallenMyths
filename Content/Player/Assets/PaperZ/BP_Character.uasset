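; Player character for a run-based PaperZD game, with axis movement, directional light attacks, a dash, a pause menu and debug keys.
; WASD state flips the sprite, repositions the attack collision and selects which combo message reaches the animation instance.
; The Dashing flag means dash ready, so damage is ignored through dash and cooldown.
; Tick checks for death, saving gold and stats to save slots and the GameInstance, then opening EndRun.
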(event EventBeginPlay
  ;[1 1 1] Begin Play
)

(event EventTick
  (params (DeltaSeconds :type Float%20%28single-precision%29))
  (bind _runloopnum (Variables|Default|GetrunLoopNum))
  ;[1 0.6347 0] Camviar tecles per if desde MoveRight per tal de que no estiguin obligats a jugar amb a i d(pd:Tambe shauria de comprovar que al mirar cap a la esquerra la colisio del atac funcioni be)
  ;;[1 1 1] Event Tick
  (CallFunction|BoxColissionDefault)
  (if (or (or (stale Input|KeyboardEvents|A _output_get) (stale Input|KeyboardEvents|D _output_get)) (or (stale Input|KeyboardEvents|W _output_get) (stale Input|KeyboardEvents|S _output_get)))
    (Variables|Default|SetIsMoving true)
    (else
      (Variables|Default|SetIsMoving false)))
  (if (<= (Variables|Default|GetplayerHealth) 0.0)
    (CallFunction|SaveGame (Variables|Default|GetSlot%20Name%20Save))
    (CallFunction|SaveRunData false)
    (Game|OpenLevel(byObjectReference) "/Game/Levels/EndRun.EndRun")
    (bind _returnvalue (SaveGame|CreateSaveGameObject "/Game/SaveLoad/SaveRun.SaveRun_C"))
    (Variables|/Game/SaveLoad/SaveRun.SaveRun_C|SetplayerGold _returnvalue (+ (Variables|Default|GetgoldAmount) (Variables|/Game/SaveLoad/SaveRun.SaveRun_C|GetplayerGold _returnvalue)))
    (if (> _runloopnum (Variables|/Game/SaveLoad/SaveRun.SaveRun_C|GetmaxNumLoop _returnvalue))
      (Variables|/Game/SaveLoad/SaveRun.SaveRun_C|SetmaxNumLoop _returnvalue _runloopnum)
      (|AsyncSaveGametoSlot _returnvalue (Variables|/Game/SaveLoad/SaveRun.SaveRun_C|GetSaveSlotName _returnvalue) (Variables|/Game/SaveLoad/SaveRun.SaveRun_C|GetplayerIndex _returnvalue)))))

(event Input|ActionEvents|InputActionHeavyAttack
  (params (Key :type Key%20Structure :default "None"))
  ;[1 1 1] Attacks
)

(event Input|ActionEvents|InputActionSprint
  (params (Key :type Key%20Structure :default "None"))
  ;[0 1 0.0648] Sprint (Walk speed i animation speed)
)

(event Input|ActionEvents|InputActionDash
  (params (Key :type Key%20Structure :default "None"))
  (bind _charactermovement (Variables|Character|GetCharacterMovement))
  ;[0.003467 1 0] Dash
  (:Pressed
    (if (and (Variables|Default|GetIsMoving) (Variables|Default|GetDashing))
      (Variables|Default|SetDashing false)
      (Variables|/Script/Engine.CharacterMovementComponent|SetMaxWalkSpeed _charactermovement 2.5e+03)
      (Class|PaperZDAnimInstance|JumptoNode (Variables|/Script/PaperZD.PaperZDAnimationComponent|GetAnimInstance (Variables|Default|GetAnimationComponent)) "Dash" "None")
      (Utilities|FlowControl|Delay 0.45)
      (Variables|/Script/Engine.CharacterMovementComponent|SetMaxWalkSpeed _charactermovement 6e+02)
      (Utilities|FlowControl|Delay 0.8)
      (Variables|Default|SetDashing true)))
  (:Released
    (Variables|/Script/Engine.CharacterMovementComponent|SetMaxWalkSpeed (Variables|Character|GetCharacterMovement) 6e+02)))

(event Input|ActionEvents|InputActionLightAttack
  (params (Key :type Key%20Structure :default "None"))
  (bind _animationcomponent (Variables|Default|GetAnimationComponent))
  (bind _animinstance (Variables|/Script/PaperZD.PaperZDAnimationComponent|GetAnimInstance _animationcomponent))
  ;[1 1 1] Attacks
  (:Pressed
    (if (Variables|Default|GetpressingW)
      (Class|BPIComboRequest+|RequestCombo(Message) _animinstance "NewEnumerator3")
      (elif (Variables|Default|GetpressingS)
        (Class|BPIComboRequest+|RequestCombo(Message) _animinstance "NewEnumerator4")
        (elif (or (or (or (or (Variables|Default|GetpressingD) (Variables|Default|GetpressingA)) (and (Variables|Default|GetpressingA) (Variables|Default|GetpressingW))) (or (and (Variables|Default|GetpressingA) (Variables|Default|GetpressingS)) (and (Variables|Default|GetpressingW) (Variables|Default|GetpressingD)))) (or (and (Variables|Default|GetpressingS) (Variables|Default|GetpressingD)) (and (and (Math|Boolean|Equal(Boolean) (Variables|Default|GetpressingW) false) (Math|Boolean|Equal(Boolean) (Variables|Default|GetpressingS) false)) (and (Math|Boolean|Equal(Boolean) (Variables|Default|GetpressingA) false) (Math|Boolean|Equal(Boolean) (Variables|Default|GetpressingD) false)))))
          (Class|BPIComboRequest+|RequestCombo(Message) _animinstance "NewEnumerator0"))))))

(event Input|AxisEvents|InputAxisMoveRight
  (params (AxisValue :type Float%20%28single-precision%29))
  (Pawn|Input|AddMovementInput "0.000000,1.000000, 0" AxisValue false))

(event Input|AxisEvents|InputAxisMoveUPDown
  (params (AxisValue :type Float%20%28single-precision%29))
  (Pawn|Input|AddMovementInput "1.000000,0.000000,0.000000" AxisValue false))

(event Input|KeyboardEvents|A
  (params (Key :type Key%20Structure :default "None"))
  (bind _runloopnum (Variables|Default|GetrunLoopNum))
  ;[1 0.6347 0] Camviar tecles per if desde MoveRight per tal de que no estiguin obligats a jugar amb a i d(pd:Tambe shauria de comprovar que al mirar cap a la esquerra la colisio del atac funcioni be)
  (:Pressed
    (Variables|Default|SetRotationDE false)
    (Transformation|SetWorldRotation (Variables|Default|GetSprite) "0,-90.000000, 0" false false)
    (Transformation|SetRelativeLocationAndRotation (Variables|Default|GetAttackCollision) "15.000000,0.000000,0.000000" "0.000000,90.000000,0.000000" false false)
    (Variables|Default|SetlastpressedA true)
    (Variables|Default|SetlastpressedD false)
    (bind _output_get (Variables|Default|SetpressingA true))
    (if (or (or _output_get (stale Input|KeyboardEvents|D _output_get)) (or (stale Input|KeyboardEvents|W _output_get) (stale Input|KeyboardEvents|S _output_get)))
      (Variables|Default|SetIsMoving true)
      (else
        (Variables|Default|SetIsMoving false)))
    ;[1 1 1] Event Tick
    (if (<= (Variables|Default|GetplayerHealth) 0.0)
      (CallFunction|SaveGame (Variables|Default|GetSlot%20Name%20Save))
      (CallFunction|SaveRunData false)
      (Game|OpenLevel(byObjectReference) "/Game/Levels/EndRun.EndRun")
      (bind _returnvalue (SaveGame|CreateSaveGameObject "/Game/SaveLoad/SaveRun.SaveRun_C"))
      (Variables|/Game/SaveLoad/SaveRun.SaveRun_C|SetplayerGold _returnvalue (+ (Variables|Default|GetgoldAmount) (Variables|/Game/SaveLoad/SaveRun.SaveRun_C|GetplayerGold _returnvalue)))
      (if (> _runloopnum (Variables|/Game/SaveLoad/SaveRun.SaveRun_C|GetmaxNumLoop _returnvalue))
        (Variables|/Game/SaveLoad/SaveRun.SaveRun_C|SetmaxNumLoop _returnvalue _runloopnum)
        (|AsyncSaveGametoSlot _returnvalue (Variables|/Game/SaveLoad/SaveRun.SaveRun_C|GetSaveSlotName _returnvalue) (Variables|/Game/SaveLoad/SaveRun.SaveRun_C|GetplayerIndex _returnvalue)))))
  (:Released
    (Variables|Default|SetpressingA false)))

(event Input|KeyboardEvents|D
  (params (Key :type Key%20Structure :default "None"))
  (bind _runloopnum (Variables|Default|GetrunLoopNum))
  ;[1 0.6347 0] Camviar tecles per if desde MoveRight per tal de que no estiguin obligats a jugar amb a i d(pd:Tambe shauria de comprovar que al mirar cap a la esquerra la colisio del atac funcioni be)
  (:Pressed
    (Variables|Default|SetRotationDE true)
    (Transformation|SetWorldRotation (Variables|Default|GetSprite) "0,90.000000, 0" false false)
    (Transformation|SetRelativeLocationAndRotation (Variables|Default|GetAttackCollision) "15.000000,0.000000,0.000000" "0.000000,90.000000,0.000000" false false)
    (Variables|Default|SetlastpressedD true)
    (Variables|Default|SetlastpressedA false)
    (bind _output_get (Variables|Default|SetpressingD true))
    (if (or (or (stale Input|KeyboardEvents|A _output_get) _output_get) (or (stale Input|KeyboardEvents|W _output_get) (stale Input|KeyboardEvents|S _output_get)))
      (Variables|Default|SetIsMoving true)
      (else
        (Variables|Default|SetIsMoving false)))
    ;[1 1 1] Event Tick
    (if (<= (Variables|Default|GetplayerHealth) 0.0)
      (CallFunction|SaveGame (Variables|Default|GetSlot%20Name%20Save))
      (CallFunction|SaveRunData false)
      (Game|OpenLevel(byObjectReference) "/Game/Levels/EndRun.EndRun")
      (bind _returnvalue (SaveGame|CreateSaveGameObject "/Game/SaveLoad/SaveRun.SaveRun_C"))
      (Variables|/Game/SaveLoad/SaveRun.SaveRun_C|SetplayerGold _returnvalue (+ (Variables|Default|GetgoldAmount) (Variables|/Game/SaveLoad/SaveRun.SaveRun_C|GetplayerGold _returnvalue)))
      (if (> _runloopnum (Variables|/Game/SaveLoad/SaveRun.SaveRun_C|GetmaxNumLoop _returnvalue))
        (Variables|/Game/SaveLoad/SaveRun.SaveRun_C|SetmaxNumLoop _returnvalue _runloopnum)
        (|AsyncSaveGametoSlot _returnvalue (Variables|/Game/SaveLoad/SaveRun.SaveRun_C|GetSaveSlotName _returnvalue) (Variables|/Game/SaveLoad/SaveRun.SaveRun_C|GetplayerIndex _returnvalue)))))
  (:Released
    (Variables|Default|SetpressingD false)))

(event Input|KeyboardEvents|W
  (params (Key :type Key%20Structure :default "None"))
  (bind _attackcollision (Variables|Default|GetAttackCollision))
  (bind _runloopnum (Variables|Default|GetrunLoopNum))
  ;[1 0.6347 0] Camviar tecles per if desde MoveRight per tal de que no estiguin obligats a jugar amb a i d(pd:Tambe shauria de comprovar que al mirar cap a la esquerra la colisio del atac funcioni be)
  (:Pressed
    (if (Variables|Default|GetRotationDE)
      (Transformation|SetRelativeLocationAndRotation _attackcollision "0.000000,-15.000000,0.000000" "0.000000,-180.000000,0.000000" false false)
      (else
        (Transformation|SetRelativeLocationAndRotation _attackcollision "0.000000,15.000000,0.000000" "0.000000,-180.000000,0.000000" false false)))
    (bind _output_get (Variables|Default|SetpressingW true))
    (if (or (or (stale Input|KeyboardEvents|A _output_get) (stale Input|KeyboardEvents|D _output_get)) (or _output_get (stale Input|KeyboardEvents|S _output_get)))
      (Variables|Default|SetIsMoving true)
      (else
        (Variables|Default|SetIsMoving false)))
    ;[1 1 1] Event Tick
    (if (<= (Variables|Default|GetplayerHealth) 0.0)
      (CallFunction|SaveGame (Variables|Default|GetSlot%20Name%20Save))
      (CallFunction|SaveRunData false)
      (Game|OpenLevel(byObjectReference) "/Game/Levels/EndRun.EndRun")
      (bind _returnvalue (SaveGame|CreateSaveGameObject "/Game/SaveLoad/SaveRun.SaveRun_C"))
      (Variables|/Game/SaveLoad/SaveRun.SaveRun_C|SetplayerGold _returnvalue (+ (Variables|Default|GetgoldAmount) (Variables|/Game/SaveLoad/SaveRun.SaveRun_C|GetplayerGold _returnvalue)))
      (if (> _runloopnum (Variables|/Game/SaveLoad/SaveRun.SaveRun_C|GetmaxNumLoop _returnvalue))
        (Variables|/Game/SaveLoad/SaveRun.SaveRun_C|SetmaxNumLoop _returnvalue _runloopnum)
        (|AsyncSaveGametoSlot _returnvalue (Variables|/Game/SaveLoad/SaveRun.SaveRun_C|GetSaveSlotName _returnvalue) (Variables|/Game/SaveLoad/SaveRun.SaveRun_C|GetplayerIndex _returnvalue)))))
  (:Released
    (Variables|Default|SetpressingW false)))

(event Input|KeyboardEvents|S
  (params (Key :type Key%20Structure :default "None"))
  (bind _attackcollision (Variables|Default|GetAttackCollision))
  (bind _runloopnum (Variables|Default|GetrunLoopNum))
  ;[1 0.6347 0] Camviar tecles per if desde MoveRight per tal de que no estiguin obligats a jugar amb a i d(pd:Tambe shauria de comprovar que al mirar cap a la esquerra la colisio del atac funcioni be)
  (:Pressed
    (if (Variables|Default|GetRotationDE)
      (Transformation|SetRelativeLocationAndRotation _attackcollision "0.000000,15.000000,0.000000" "0.000000,-180.000000,0.000000" false false)
      (else
        (Transformation|SetRelativeLocationAndRotation _attackcollision "0.000000,-15.000000,0.000000" "0.000000,-180.000000,0.000000" false false)))
    (bind _output_get (Variables|Default|SetpressingS true))
    (if (or (or (stale Input|KeyboardEvents|A _output_get) (stale Input|KeyboardEvents|D _output_get)) (or (stale Input|KeyboardEvents|W _output_get) _output_get))
      (Variables|Default|SetIsMoving true)
      (else
        (Variables|Default|SetIsMoving false)))
    ;[1 1 1] Event Tick
    (if (<= (Variables|Default|GetplayerHealth) 0.0)
      (CallFunction|SaveGame (Variables|Default|GetSlot%20Name%20Save))
      (CallFunction|SaveRunData false)
      (Game|OpenLevel(byObjectReference) "/Game/Levels/EndRun.EndRun")
      (bind _returnvalue (SaveGame|CreateSaveGameObject "/Game/SaveLoad/SaveRun.SaveRun_C"))
      (Variables|/Game/SaveLoad/SaveRun.SaveRun_C|SetplayerGold _returnvalue (+ (Variables|Default|GetgoldAmount) (Variables|/Game/SaveLoad/SaveRun.SaveRun_C|GetplayerGold _returnvalue)))
      (if (> _runloopnum (Variables|/Game/SaveLoad/SaveRun.SaveRun_C|GetmaxNumLoop _returnvalue))
        (Variables|/Game/SaveLoad/SaveRun.SaveRun_C|SetmaxNumLoop _returnvalue _runloopnum)
        (|AsyncSaveGametoSlot _returnvalue (Variables|/Game/SaveLoad/SaveRun.SaveRun_C|GetSaveSlotName _returnvalue) (Variables|/Game/SaveLoad/SaveRun.SaveRun_C|GetplayerIndex _returnvalue)))))
  (:Released
    (Variables|Default|SetpressingS false)))

(event Input|KeyboardEvents|CCedille
  (params (Key :type Key%20Structure :default "None"))
  ;[1 0 0.03099] Treure
  (:Pressed
    (Game|OpenLevel(byObjectReference) "/Game/Levels/EndRun.EndRun")))

(event Input|KeyboardEvents|+
  (params (Key :type Key%20Structure :default "None"))
  ;[1 0 0.03099] Treure
  (:Pressed
    (CallFunction|GetDamage 0.07)))

(event Input|KeyboardEvents|Escape
  (params (Key :type Key%20Structure :default "None"))
  (bind _returnvalue (Game|GetPlayerController 0))
  ;[1 1 1] Pause Menu
  (:Pressed
    (Utilities|IsValid (Variables|Default|GetrefPauseMenu)
      (:Is%20Valid
        _)
      (:Is%20Not%20Valid
        (bind _returnvalue_2 (UserInterface|CreateWidget "/Game/UI/UI_PauseMenuInGame.UI_PauseMenuInGame_C"))
        (Variables|Default|SetrefPauseMenu _returnvalue_2)))
    (Variables|/Script/Engine.PlayerController|SetbShowMouseCursor _returnvalue true)
    (Input|SetInputModeUIOnly _returnvalue (Variables|Default|GetrefPauseMenu) "DoNotLock")
    (UserInterface|Viewport|AddtoViewport (Variables|Default|GetrefPauseMenu) 0)
    (Game|SetGamePaused true)))

(event Input|KeyboardEvents|P
  (params (Key :type Key%20Structure :default "None"))
  (bind _returnvalue (Game|GetPlayerController 0))
  ;[1 1 1] Pause Menu
  (:Pressed
    (Utilities|IsValid (Variables|Default|GetrefPauseMenu)
      (:Is%20Valid
        _)
      (:Is%20Not%20Valid
        (bind _returnvalue_2 (UserInterface|CreateWidget "/Game/UI/UI_PauseMenuInGame.UI_PauseMenuInGame_C"))
        (Variables|Default|SetrefPauseMenu _returnvalue_2)))
    (Variables|/Script/Engine.PlayerController|SetbShowMouseCursor _returnvalue true)
    (Input|SetInputModeUIOnly _returnvalue (Variables|Default|GetrefPauseMenu) "DoNotLock")
    (UserInterface|Viewport|AddtoViewport (Variables|Default|GetrefPauseMenu) 0)
    (Game|SetGamePaused true)))

(event Input|KeyboardEvents|Tab
  (params (Key :type Key%20Structure :default "None"))
  ;[1 1 1] Pause Menu
)

(fn ConstructionScript)

(fn Teleportto
  (params (newPosition :type Vector))
  (bind (_x _y _z) (Math|Vector|BreakVector newPosition))
  (Transformation|SetActorLocation (Math|Vector|MakeVector _x _y (+ _z 63.0)) false false))

(fn MoveCam
  (params (Direction :type Integer))
  ;[1 1 1 1 16] Segons l'int movem la camera en una de les 4 direccions
  ; 1 = nord, 2= sud, 3 = est, 4 = oest
)

(fn SetRoomXY
  (params (_x :type Integer) (_y :type Integer))
  (Variables|Default|SetroomX _x)
  (Variables|Default|SetroomY _y))

(fn SaveRunData
  (params (playerWon :type Boolean))
  (bind _asmy_game_instance (Utilities|Casting|CastToMyGameInstance (Game|GetGameInstance)))
  (bind _asbp_character (Utilities|Casting|CastToBP_Character (Game|Player|GetPlayerPawn 0)))
  (Utilities|FlowControl|Sequence
    (:then_0
      (Variables|/Game/SaveLoad/MyGameInstance.MyGameInstance_C|SetenemiesKilled _asmy_game_instance (Variables|BP_Character_C|GetenemiesKilled _asbp_character)))
    (:then_1
      (Variables|/Game/SaveLoad/MyGameInstance.MyGameInstance_C|SetdmgTaken _asmy_game_instance (Variables|BP_Character_C|GetdmgTaken _asbp_character)))
    (:then_2
      (Variables|/Game/SaveLoad/MyGameInstance.MyGameInstance_C|SetgoldAmount _asmy_game_instance (Variables|BP_Character_C|GetgoldAmount _asbp_character)))
    (:then_3
      (Variables|/Game/SaveLoad/MyGameInstance.MyGameInstance_C|SetlastTime _asmy_game_instance 0))
    (:then_4
      (if playerWon
        (Variables|/Game/SaveLoad/MyGameInstance.MyGameInstance_C|SetrunLoopNum _asmy_game_instance (+ (Variables|BP_Character_C|GetrunLoopNum _asbp_character) 1))
        (else
          (Variables|/Game/SaveLoad/MyGameInstance.MyGameInstance_C|SetrunLoopNum _asmy_game_instance (Variables|BP_Character_C|GetrunLoopNum _asbp_character)))))
    (:then_5
      (if (<= (Variables|BP_Character_C|GetplayerHealth _asbp_character) 0.0)
        (Variables|/Game/SaveLoad/MyGameInstance.MyGameInstance_C|SetplayerHealth _asmy_game_instance 1.0)
        (else
          (Variables|/Game/SaveLoad/MyGameInstance.MyGameInstance_C|SetplayerHealth _asmy_game_instance (Variables|BP_Character_C|GetplayerHealth _asbp_character)))))
    (:then_6
      (Variables|/Game/SaveLoad/MyGameInstance.MyGameInstance_C|SetdamageReduction _asmy_game_instance (Variables|Default|GetdamageReduction)))))

(fn GetDamage
  (params (dmgAmount :type Float%20%28single-precision%29))
  (if (Variables|Default|GetDashing)
    (bind _output_get (Variables|Default|SetplayerHealth (- (Variables|Default|GetplayerHealth) (* dmgAmount (Variables|Default|GetdamageReduction)))))
    (Variables|Default|SetdmgTaken (+ dmgAmount (Variables|Default|GetdmgTaken)))
    (Development|PrintString (Utilities|String|ToString(Float) _output_get) true true "(R=1.000000,G=0.000000,B=0.235368,A=1.000000)")))

(fn HealthUp
  (Variables|Default|SetplayerHealth 1.0))

(fn LoadRunData
  (bind _asmy_game_instance (Utilities|Casting|CastToMyGameInstance (Game|GetGameInstance)))
  (Utilities|FlowControl|Sequence
    (:then_0
      (Variables|Default|SetdmgTaken (Variables|/Game/SaveLoad/MyGameInstance.MyGameInstance_C|GetdmgTaken _asmy_game_instance)))
    (:then_1
      (Variables|Default|SetenemiesKilled (Variables|/Game/SaveLoad/MyGameInstance.MyGameInstance_C|GetenemiesKilled _asmy_game_instance)))
    (:then_2
      (Variables|Default|SetgoldAmount (Variables|/Game/SaveLoad/MyGameInstance.MyGameInstance_C|GetgoldAmount _asmy_game_instance)))
    (:then_3
      (Variables|Default|SetrunLoopNum (Variables|/Game/SaveLoad/MyGameInstance.MyGameInstance_C|GetrunLoopNum _asmy_game_instance)))
    (:then_4
      (Variables|Default|SetplayerHealth (Variables|/Game/SaveLoad/MyGameInstance.MyGameInstance_C|GetplayerHealth _asmy_game_instance)))
    (:then_5
      (Variables|Default|SetdamageReduction (Variables|/Game/SaveLoad/MyGameInstance.MyGameInstance_C|GetdamageReduction _asmy_game_instance)))))

(fn ResetDash)

(fn SaveGame
  (params (SlotName :type String))
  (bind _returnvalue (SaveGame|DoesSaveGameExist SlotName))
  (if _returnvalue
    (bind _returnvalue_2 (SaveGame|LoadGamefromSlot SlotName))
    (Variables|Default|SetSave%20REF _returnvalue_2)
    (else
      (bind _returnvalue_3 (SaveGame|CreateSaveGameObject "/Game/SaveLoad/SaveGame.SaveGame_C"))
      (bind _output_get (Variables|Default|SetSave%20REF _returnvalue_3))))
  (bind _assave_game (Utilities|Casting|CastToSaveGame _output_get))
  (Variables|/Game/SaveLoad/SaveGame.SaveGame_C|SetGold _assave_game (Variables|Default|GetgoldAmount))
  ;[1 1 1] Guardar vida
  (Variables|/Game/SaveLoad/SaveGame.SaveGame_C|SetDamageReduciton _assave_game (Variables|Default|GetdamageReduction))
  (bind _asmy_game_instance (Utilities|Casting|CastToMyGameInstance (Game|GetGameInstance)))
  (Variables|/Game/SaveLoad/MyGameInstance.MyGameInstance_C|SetgoldAmount _asmy_game_instance (Variables|Default|GetgoldAmount))
  ;[1 1 1] Comment
  (Variables|/Game/SaveLoad/MyGameInstance.MyGameInstance_C|SetdamageReduction _asmy_game_instance (Variables|Default|GetdamageReduction))
  (SaveGame|SaveGametoSlot (Variables|Default|GetSave%20REF) SlotName))

(fn LoadGame
  (params (SlotName :type String))
  (bind _returnvalue (SaveGame|DoesSaveGameExist SlotName))
  (if _returnvalue
    (bind _returnvalue_2 (SaveGame|LoadGamefromSlot SlotName))
    (bind _assave_game (Utilities|Casting|CastToSaveGame _returnvalue_2))
    (bind _output_get (Variables|Default|SetgoldAmount (Variables|/Game/SaveLoad/SaveGame.SaveGame_C|GetGold _assave_game)))
    (bind _asmy_game_instance (Utilities|Casting|CastToMyGameInstance (Game|GetGameInstance)))
    (Variables|/Game/SaveLoad/MyGameInstance.MyGameInstance_C|SetgoldAmount _asmy_game_instance _output_get)))

(fn BoxColissionDefault
  (bind _pressingw (Variables|Default|GetpressingW))
  (bind _attackcollision (Variables|Default|GetAttackCollision))
  (bind _pressings (Variables|Default|GetpressingS))
  (bind _pressinga (Variables|Default|GetpressingA))
  (bind _pressingd (Variables|Default|GetpressingD))
  (bind _sprite (Variables|Default|GetSprite))
  (bind _returnvalue (Math|Boolean|Equal(Boolean) _pressingd false))
  (bind _returnvalue_2 (Math|Boolean|Equal(Boolean) _pressingw false))
  (bind _returnvalue_3 (Math|Boolean|Equal(Boolean) _pressings false))
  (bind _returnvalue_4 (Math|Boolean|Equal(Boolean) _pressinga false))
  (bind _returnvalue_5 (and _returnvalue_2 _returnvalue_3))
  (bind _returnvalue_6 (and _returnvalue_4 _returnvalue))
  (bind _returnvalue_7 (and _returnvalue_5 _returnvalue_6))
  (if (Math|Boolean|Equal(Boolean) (Variables|Default|GetlastpressedA) true)
    (if _returnvalue_7
      (Transformation|SetWorldRotation _sprite "0,-90.000000, 0" false false)
      (Transformation|SetRelativeLocationAndRotation _attackcollision "15.000000,0.000000,0.000000" "0.000000,-90.000000,0.000000" false false))
    (elif _returnvalue_7
      (Transformation|SetWorldRotation _sprite "0,90.000000, 0" false false)
      (Transformation|SetRelativeLocationAndRotation _attackcollision "15.000000,0.000000,0.000000" "0.000000,90.000000,0.000000" false false))))