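; Base room actor for the procedurally generated grid map, linked to up to four neighbours.
; ModifyDoors reads a 4-bit door mask to show bridges and disable unused edge colliders.
; Edge overlaps teleport the player to the neighbour, switch camera, update minimap and lock further teleports while that room's enemy count is above zero.
; The construction script scatters randomised instanced leaf meshes without collision.
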(event OnComponentBeginOverlap(NorthCollider)
  (params (OverlappedComponent :type Primitive%20Component%20Object%20Reference) (OtherActor :type Actor%20Object%20Reference) (OtherComp :type Primitive%20Component%20Object%20Reference) (OtherBodyIndex :type Integer) (bFromSweep :type Boolean) (SweepResult :type Hit%20Result%20Structure%20%28by%20ref%29))
  (bind _returnvalue (Game|Player|GetPlayerPawn 0))
  (bind _northroom (Variables|Default|GetNorthRoom))
  (bind _northroom_2 (Variables|Default|GetNorthRoom))
  ;[1 1 1] Nord
  (if (== OtherActor _returnvalue)
    (bind _asbp_character (Utilities|Casting|CastToBP_Character _returnvalue)
      (:then
        (if (Variables|/Game/Player/Assets/PaperZ/BP_Character.BP_Character_C|GetcanTP _asbp_character)
          (Transformation|SetActorLocation _returnvalue (Transformation|GetWorldLocation (Variables|BaseGeneralRoom_C|GetSouthPoint _northroom_2)) false false)
          (bind _asbp_character_2 (Utilities|Casting|CastToBP_Character _returnvalue))
          (Default|ChangeCamera (Variables|Default|GetrefCamManager) (Variables|BaseGeneralRoom_C|GetroomX _northroom_2) (Variables|BaseGeneralRoom_C|GetroomY _northroom_2))
          (Variables|/Game/Player/Assets/PaperZ/BP_Character.BP_Character_C|SetcanTP _asbp_character_2 false)
          (Math|Integer|DecrementInt (Variables|/Game/Player/Assets/PaperZ/BP_Character.BP_Character_C|GetroomY _asbp_character_2)
            (:%20%20
              ;;[1 1 1] Cridem a la següent sala
              (CallFunction|PlayerEnters _northroom)
              (Variables|BaseGeneralRoom_C|Setdescoberta _northroom true)
              (bind _asbp_character_3 (Utilities|Casting|CastToBP_Character (Game|Player|GetPlayerPawn 0)))
              (bind _asmini_map (Utilities|Casting|CastToMiniMap (Variables|/Game/Player/Assets/PaperZ/BP_Character.BP_Character_C|GetrefMiniMap _asbp_character_3)))
              (Default|CheckRoomsSeen _asmini_map)
              (CallFunction|CheckAmountEnemies _northroom)))))
      (:CastFailed
        (Development|PrintString "Not Cast" true true "(R=1.000000,G=0.000000,B=0.871570,A=1.000000)")))))

(event OnComponentBeginOverlap(SouthCollider)
  (params (OverlappedComponent :type Primitive%20Component%20Object%20Reference) (OtherActor :type Actor%20Object%20Reference) (OtherComp :type Primitive%20Component%20Object%20Reference) (OtherBodyIndex :type Integer) (bFromSweep :type Boolean) (SweepResult :type Hit%20Result%20Structure%20%28by%20ref%29))
  (bind _returnvalue (Game|Player|GetPlayerPawn 0))
  (bind _southroom (Variables|Default|GetSouthRoom))
  (bind _southroom_2 (Variables|Default|GetSouthRoom))
  ;[1 1 1] Sud
  (if (== OtherActor _returnvalue)
    (bind _asbp_character (Utilities|Casting|CastToBP_Character _returnvalue)
      (:then
        (if (Variables|/Game/Player/Assets/PaperZ/BP_Character.BP_Character_C|GetcanTP _asbp_character)
          (Transformation|SetActorLocation _returnvalue (Transformation|GetWorldLocation (Variables|BaseGeneralRoom_C|GetNorthPoint _southroom_2)) false false)
          (bind _asbp_character_2 (Utilities|Casting|CastToBP_Character _returnvalue))
          (Default|ChangeCamera (Variables|Default|GetrefCamManager) (Variables|BaseGeneralRoom_C|GetroomX _southroom_2) (Variables|BaseGeneralRoom_C|GetroomY _southroom_2))
          (Variables|/Game/Player/Assets/PaperZ/BP_Character.BP_Character_C|SetcanTP _asbp_character_2 false)
          (Math|Integer|IncrementInt (Variables|/Game/Player/Assets/PaperZ/BP_Character.BP_Character_C|GetroomY _asbp_character_2)
            (:%20%20
              ;;[1 1 1] Cridem a la següent sala
              (CallFunction|PlayerEnters _southroom)
              (Variables|BaseGeneralRoom_C|Setdescoberta _southroom true)
              (bind _asbp_character_3 (Utilities|Casting|CastToBP_Character (Game|Player|GetPlayerPawn 0)))
              (bind _asmini_map (Utilities|Casting|CastToMiniMap (Variables|/Game/Player/Assets/PaperZ/BP_Character.BP_Character_C|GetrefMiniMap _asbp_character_3)))
              (Default|CheckRoomsSeen _asmini_map)
              (CallFunction|CheckAmountEnemies _southroom)))))
      (:CastFailed
        (Development|PrintString "Not Cast" true true "(R=1.000000,G=0.000000,B=0.871570,A=1.000000)")))))

(event OnComponentHit(EastCollider)
  (params (HitComponent :type Primitive%20Component%20Object%20Reference) (OtherActor :type Actor%20Object%20Reference) (OtherComp :type Primitive%20Component%20Object%20Reference) (NormalImpulse :type Vector :default "0, 0, 0") (Hit :type Hit%20Result%20Structure%20%28by%20ref%29))
  ;[1 1 1] Est
  ;;[1 1 1 1 16] Aquesta zona no funciona, ens mou el jugador diverses vegades, muiltiples print string
)

(event OnComponentBeginOverlap(EastCollider)
  (params (OverlappedComponent :type Primitive%20Component%20Object%20Reference) (OtherActor :type Actor%20Object%20Reference) (OtherComp :type Primitive%20Component%20Object%20Reference) (OtherBodyIndex :type Integer) (bFromSweep :type Boolean) (SweepResult :type Hit%20Result%20Structure%20%28by%20ref%29))
  (bind _returnvalue (Game|Player|GetPlayerPawn 0))
  (bind _eastroom (Variables|Default|GetEastRoom))
  (bind _eastroom_2 (Variables|Default|GetEastRoom))
  ;[1 1 1] Est
  ;;[1 1 1 1 16] Aquesta zona no funciona, ens mou el jugador diverses vegades, muiltiples print string
  (if (== OtherActor _returnvalue)
    (bind _asbp_character (Utilities|Casting|CastToBP_Character _returnvalue)
      (:then
        (if (Variables|/Game/Player/Assets/PaperZ/BP_Character.BP_Character_C|GetcanTP _asbp_character)
          (Transformation|SetActorLocation _returnvalue (Transformation|GetWorldLocation (Variables|BaseGeneralRoom_C|GetWestPoint _eastroom)) false true)
          (bind _asbp_character_2 (Utilities|Casting|CastToBP_Character _returnvalue))
          (Default|ChangeCamera (Variables|Default|GetrefCamManager) (Variables|BaseGeneralRoom_C|GetroomX _eastroom) (Variables|BaseGeneralRoom_C|GetroomY _eastroom))
          (Variables|/Game/Player/Assets/PaperZ/BP_Character.BP_Character_C|SetcanTP _asbp_character_2 false)
          (Math|Integer|IncrementInt (Variables|/Game/Player/Assets/PaperZ/BP_Character.BP_Character_C|GetroomX _asbp_character_2)
            (:%20%20
              ;;[1 1 1] Cridem a la següent sala
              (CallFunction|PlayerEnters _eastroom_2)
              (Variables|BaseGeneralRoom_C|Setdescoberta _eastroom_2 true)
              (bind _asbp_character_3 (Utilities|Casting|CastToBP_Character (Game|Player|GetPlayerPawn 0)))
              (bind _asmini_map (Utilities|Casting|CastToMiniMap (Variables|/Game/Player/Assets/PaperZ/BP_Character.BP_Character_C|GetrefMiniMap _asbp_character_3)))
              (Default|CheckRoomsSeen _asmini_map)
              (CallFunction|CheckAmountEnemies _eastroom_2)))))
      (:CastFailed
        (Development|PrintString "Not Cast" true true "(R=1.000000,G=0.000000,B=0.871570,A=1.000000)")))))

(event OnComponentHit(NorthCollider)
  (params (HitComponent :type Primitive%20Component%20Object%20Reference) (OtherActor :type Actor%20Object%20Reference) (OtherComp :type Primitive%20Component%20Object%20Reference) (NormalImpulse :type Vector :default "0, 0, 0") (Hit :type Hit%20Result%20Structure%20%28by%20ref%29))
  ;[1 1 1] Nord
)

(event OnComponentBeginOverlap(WestCollider)
  (params (OverlappedComponent :type Primitive%20Component%20Object%20Reference) (OtherActor :type Actor%20Object%20Reference) (OtherComp :type Primitive%20Component%20Object%20Reference) (OtherBodyIndex :type Integer) (bFromSweep :type Boolean) (SweepResult :type Hit%20Result%20Structure%20%28by%20ref%29))
  (bind _returnvalue (Game|Player|GetPlayerPawn 0))
  (bind _westroom (Variables|Default|GetWestRoom))
  (bind _westroom_2 (Variables|Default|GetWestRoom))
  ;[1 1 1] Oest
  (if (== OtherActor _returnvalue)
    (bind _asbp_character (Utilities|Casting|CastToBP_Character _returnvalue)
      (:then
        (if (Variables|/Game/Player/Assets/PaperZ/BP_Character.BP_Character_C|GetcanTP _asbp_character)
          (Transformation|SetActorLocation _returnvalue (Transformation|GetWorldLocation (Variables|BaseGeneralRoom_C|GetEastPoint _westroom)) false false)
          (bind _asbp_character_2 (Utilities|Casting|CastToBP_Character _returnvalue))
          (Default|ChangeCamera (Variables|Default|GetrefCamManager) (Variables|BaseGeneralRoom_C|GetroomX _westroom) (Variables|BaseGeneralRoom_C|GetroomY _westroom))
          (Variables|/Game/Player/Assets/PaperZ/BP_Character.BP_Character_C|SetcanTP _asbp_character_2 false)
          (Math|Integer|DecrementInt (Variables|/Game/Player/Assets/PaperZ/BP_Character.BP_Character_C|GetroomX _asbp_character_2)
            (:%20%20
              ;;[1 1 1] Cridem a la següent sala
              (CallFunction|PlayerEnters _westroom_2)
              (Variables|BaseGeneralRoom_C|Setdescoberta _westroom_2 true)
              (bind _asbp_character_3 (Utilities|Casting|CastToBP_Character (Game|Player|GetPlayerPawn 0)))
              (bind _asmini_map (Utilities|Casting|CastToMiniMap (Variables|/Game/Player/Assets/PaperZ/BP_Character.BP_Character_C|GetrefMiniMap _asbp_character_3)))
              (Default|CheckRoomsSeen _asmini_map)
              (CallFunction|CheckAmountEnemies _westroom_2)))))
      (:CastFailed
        (Development|PrintString "Not Cast" true true "(R=1.000000,G=0.000000,B=0.871570,A=1.000000)")))))

(event OnComponentHit(SouthCollider)
  (params (HitComponent :type Primitive%20Component%20Object%20Reference) (OtherActor :type Actor%20Object%20Reference) (OtherComp :type Primitive%20Component%20Object%20Reference) (NormalImpulse :type Vector :default "0, 0, 0") (Hit :type Hit%20Result%20Structure%20%28by%20ref%29))
  ;[1 1 1] Sud
)

(event OnComponentHit(WestCollider)
  (params (HitComponent :type Primitive%20Component%20Object%20Reference) (OtherActor :type Actor%20Object%20Reference) (OtherComp :type Primitive%20Component%20Object%20Reference) (NormalImpulse :type Vector :default "0, 0, 0") (Hit :type Hit%20Result%20Structure%20%28by%20ref%29))
  ;[1 1 1] Oest
)

(fn ConstructionScript
  (bind _distance (Variables|Default|GetDistance))
  (bind _distancernd (Variables|Default|GetDistanceRND))
  (bind _distance_2 (Variables|Default|GetDistance))
  (bind _distancernd_2 (Variables|Default|GetDistanceRND))
  (bind _rotationrnd (Variables|Default|GetRotationRND))
  (bind _scalernd (Variables|Default|GetScaleRND))
  (bind _returnvalue (AddComponent|AddInstancedStaticMeshComponent (Components|GetOwner (Variables|Default|GetLEAVES)) false))
  (Collision|SetCollisionEnabled _returnvalue "NoCollision")
  (for _index (range 0 (Variables|Default|GetSize))
    (for _index_2 (range 0 (Variables|Default|GetSize))
      (Components|InstancedStaticMesh|AddInstance _returnvalue (Math|Transform|MakeRelativeTransform (Math|Transform|MakeTransform (Math|Vector|MakeVector (+ (* _index_2 _distance) (* _distance (Math|Random|RandomFloatinRange (* _distancernd -1.0) _distancernd))) (+ (* _index _distance_2) (* _distance_2 (Math|Random|RandomFloatinRange (* _distancernd_2 -1.0) _distancernd_2))) 0.0) (Math|Rotator|MakeRotator 0.0 0.0 (Math|Random|RandomFloatinRange (* _rotationrnd -1.0) _rotationrnd)) (Math|Conversions|ToVector(Float) (+ (Math|Random|RandomFloatinRange (* _scalernd -1.0) _scalernd) 1.0))) (Math|Transform|MakeTransform "700.000000,700.000000, 0" "0, 0, 0" "0.990000,0.800000,1"))))))

(fn ModifyDoors
  (params (nDoors :type Integer))
  (bind _output_get (Variables|Default|Set_nDoors nDoors))
  (if (and (< _output_get 16) (> _output_get 0))
    (if (== (Variables|Default|Get_nDoors) 1)
      (Rendering|SetVisibility (Variables|Default|GetNorthBridge) true false)
      (Collision|SetCollisionEnabled (Variables|Default|GetSouthCollider) "NoCollision")
      (Collision|SetCollisionEnabled (Variables|Default|GetEastCollider) "NoCollision")
      (Collision|SetCollisionEnabled (Variables|Default|GetWestCollider) "NoCollision")
      (elif (== (Variables|Default|Get_nDoors) 2)
        (Rendering|SetVisibility (Variables|Default|GetSouthBridge) true false)
        (Collision|SetCollisionEnabled (Variables|Default|GetNorthCollider) "NoCollision")
        (Collision|SetCollisionEnabled (Variables|Default|GetEastCollider) "NoCollision")
        (Collision|SetCollisionEnabled (Variables|Default|GetWestCollider) "NoCollision")
        (elif (== (Variables|Default|Get_nDoors) 3)
          (Rendering|SetVisibility (Variables|Default|GetNorthBridge) true false)
          (Rendering|SetVisibility (Variables|Default|GetSouthBridge) true false)
          (Collision|SetCollisionEnabled (Variables|Default|GetEastCollider) "NoCollision")
          (Collision|SetCollisionEnabled (Variables|Default|GetWestCollider) "NoCollision")
          (elif (== (Variables|Default|Get_nDoors) 4)
            (Rendering|SetVisibility (Variables|Default|GetEastBridge) true false)
            (Collision|SetCollisionEnabled (Variables|Default|GetNorthCollider) "NoCollision")
            (Collision|SetCollisionEnabled (Variables|Default|GetSouthCollider) "NoCollision")
            (Collision|SetCollisionEnabled (Variables|Default|GetWestCollider) "NoCollision")
            (elif (== (Variables|Default|Get_nDoors) 5)
              (Rendering|SetVisibility (Variables|Default|GetNorthBridge) true false)
              (Rendering|SetVisibility (Variables|Default|GetEastBridge) true false)
              (Collision|SetCollisionEnabled (Variables|Default|GetSouthCollider) "NoCollision")
              (Collision|SetCollisionEnabled (Variables|Default|GetWestCollider) "NoCollision")
              (elif (== (Variables|Default|Get_nDoors) 6)
                (Rendering|SetVisibility (Variables|Default|GetEastBridge) true false)
                (Rendering|SetVisibility (Variables|Default|GetSouthBridge) true false)
                (Collision|SetCollisionEnabled (Variables|Default|GetNorthCollider) "NoCollision")
                (Collision|SetCollisionEnabled (Variables|Default|GetWestCollider) "NoCollision")
                (elif (== (Variables|Default|Get_nDoors) 7)
                  (Rendering|SetVisibility (Variables|Default|GetNorthBridge) true false)
                  (Rendering|SetVisibility (Variables|Default|GetEastBridge) true false)
                  (Rendering|SetVisibility (Variables|Default|GetSouthBridge) true false)
                  (Collision|SetCollisionEnabled (Variables|Default|GetWestCollider) "NoCollision")
                  (elif (== (Variables|Default|Get_nDoors) 8)
                    (Rendering|SetVisibility (Variables|Default|GetWestBridge) true false)
                    (Collision|SetCollisionEnabled (Variables|Default|GetNorthCollider) "NoCollision")
                    (Collision|SetCollisionEnabled (Variables|Default|GetSouthCollider) "NoCollision")
                    (Collision|SetCollisionEnabled (Variables|Default|GetEastCollider) "NoCollision")
                    (elif (== (Variables|Default|Get_nDoors) 9)
                      (Rendering|SetVisibility (Variables|Default|GetNorthBridge) true false)
                      (Rendering|SetVisibility (Variables|Default|GetWestBridge) true false)
                      (Collision|SetCollisionEnabled (Variables|Default|GetSouthCollider) "NoCollision")
                      (Collision|SetCollisionEnabled (Variables|Default|GetEastCollider) "NoCollision")
                      (elif (== (Variables|Default|Get_nDoors) 10)
                        (Rendering|SetVisibility (Variables|Default|GetWestBridge) true false)
                        (Rendering|SetVisibility (Variables|Default|GetSouthBridge) true false)
                        (Collision|SetCollisionEnabled (Variables|Default|GetNorthCollider) "NoCollision")
                        (Collision|SetCollisionEnabled (Variables|Default|GetEastCollider) "NoCollision")
                        (elif (== (Variables|Default|Get_nDoors) 11)
                          (Rendering|SetVisibility (Variables|Default|GetNorthBridge) true false)
                          (Rendering|SetVisibility (Variables|Default|GetWestBridge) true false)
                          (Rendering|SetVisibility (Variables|Default|GetSouthBridge) true false)
                          (Collision|SetCollisionEnabled (Variables|Default|GetEastCollider) "NoCollision")
                          (elif (== (Variables|Default|Get_nDoors) 12)
                            (Rendering|SetVisibility (Variables|Default|GetEastBridge) true false)
                            (Rendering|SetVisibility (Variables|Default|GetWestBridge) true false)
                            (Collision|SetCollisionEnabled (Variables|Default|GetNorthCollider) "NoCollision")
                            (Collision|SetCollisionEnabled (Variables|Default|GetSouthCollider) "NoCollision")
                            (elif (== (Variables|Default|Get_nDoors) 13)
                              (Rendering|SetVisibility (Variables|Default|GetNorthBridge) true false)
                              (Rendering|SetVisibility (Variables|Default|GetEastBridge) true false)
                              (Rendering|SetVisibility (Variables|Default|GetWestBridge) true false)
                              (Collision|SetCollisionEnabled (Variables|Default|GetSouthCollider) "NoCollision")
                              (elif (== (Variables|Default|Get_nDoors) 14)
                                (Rendering|SetVisibility (Variables|Default|GetSouthBridge) true false)
                                (Rendering|SetVisibility (Variables|Default|GetEastBridge) true false)
                                (Rendering|SetVisibility (Variables|Default|GetWestBridge) true false)
                                (Collision|SetCollisionEnabled (Variables|Default|GetNorthCollider) "NoCollision")
                                (elif (== (Variables|Default|Get_nDoors) 15)
                                  (Rendering|SetVisibility (Variables|Default|GetNorthBridge) true false)
                                  (Rendering|SetVisibility (Variables|Default|GetSouthBridge) true false)
                                  (Rendering|SetVisibility (Variables|Default|GetEastBridge) true false)
                                  (Rendering|SetVisibility (Variables|Default|GetWestBridge) true false))))))))))))))))))

(fn SetNorthRoom
  (params (_room :type Base%20General%20Room%20Object%20Reference))
  (Variables|Default|SetNorthRoom _room))

(fn SetSouthRoom
  (params (_room :type Base%20General%20Room%20Object%20Reference))
  (Variables|Default|SetSouthRoom _room))

(fn SetEastRoom
  (params (_room :type Base%20General%20Room%20Object%20Reference))
  (Variables|Default|SetEastRoom _room))

(fn SetWestRoom
  (params (_room :type Base%20General%20Room%20Object%20Reference))
  (Variables|Default|SetWestRoom _room))

(fn SetRoomXY
  (params (_x :type Integer) (_y :type Integer))
  (bind _output_get (Variables|Default|SetroomX _x))
  (bind _output_get_2 (Variables|Default|SetroomY _y))
  (Rendering|Components|TextRender|SetText (Variables|Default|GetText) (Utilities|Text|ToText(String) (Utilities|String|Append (Utilities|String|Append (Utilities|String|ToString(Integer) _output_get) ",") (Utilities|String|ToString(Integer) _output_get_2)))))

(fn PlayerEnters
  (Development|PrintString (Utilities|String|Append "To: " (Utilities|String|Append (Utilities|String|Append (Utilities|String|ToString(Integer) (Variables|Default|GetroomX)) ",") (Utilities|String|ToString(Integer) (Variables|Default|GetroomY)))) true true "(R=0.144696,G=0.734375,B=0.000000,A=1.000000)" 5.0))

(fn EnemyDead
  (Math|Integer|DecrementInt (Variables|Default|GetactualEnemies)))

(fn EnemySetup
  (params (_newEnemy :type Pawn%20Object%20Reference))
  (bind _aspersecutor (Utilities|Casting|CastToPersecutor _newEnemy)
    (:then
      (Variables|/Game/enemy/BaseEnemics.BaseEnemics_C|SetEnemyRoom _aspersecutor self))
    (:CastFailed
      (bind _asgorgona_petita_torreta (Utilities|Casting|CastToGorgonaPetitaTorreta _newEnemy))
      (Variables|/Game/enemy/BaseEnemics.BaseEnemics_C|SetEnemyRoom _asgorgona_petita_torreta self)
      (Math|Integer|IncrementInt (Variables|Default|GetactualEnemies)))))

(fn CheckAmountEnemies
  (bind _returnvalue (Game|Player|GetPlayerPawn 0))
  (if (<= (Variables|Default|GetactualEnemies) 0)
    (bind _asbp_character (Utilities|Casting|CastToBP_Character _returnvalue))
    (Variables|/Game/Player/Assets/PaperZ/BP_Character.BP_Character_C|SetcanTP _asbp_character true)
    (else
      (bind _asbp_character_2 (Utilities|Casting|CastToBP_Character _returnvalue))
      (Variables|/Game/Player/Assets/PaperZ/BP_Character.BP_Character_C|SetcanTP _asbp_character_2 false))))