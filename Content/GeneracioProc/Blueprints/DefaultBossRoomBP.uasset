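; Boss room Blueprint for a procedurally generated run, handling entry, enemy tracking and run exits.
; First entry raises the west door and flags the boss spawn.
; Enemy setup links each known enemy type to the room and counts it; a check raises the next-level door when none remain.
; Exit triggers save and end the run, continue to level generation until the loop limit, or teleport the player back and switch camera.
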(event OnComponentBeginOverlap(GoBackCol)
  (params (OverlappedComponent :type Primitive%20Component%20Object%20Reference) (OtherActor :type Actor%20Object%20Reference) (OtherComp :type Primitive%20Component%20Object%20Reference) (OtherBodyIndex :type Integer) (bFromSweep :type Boolean) (SweepResult :type Hit%20Result%20Structure%20%28by%20ref%29))
  (bind _returnvalue (Game|Player|GetPlayerPawn 0))
  ;[1 1 1] Player TP to final
  (Development|PrintString "Colliison" true true "(R=1.000000,G=0.000000,B=0.871570,A=1.000000)")
  (if (== OtherActor _returnvalue)
    (bind _ascharacter (Utilities|Casting|CastToCharacter _returnvalue))
    (Transformation|SetActorLocation _ascharacter (Variables|Default|GetpreBossRoom) false false)
    (CallFunction|PlayerGoBack)
    (else
      (Development|PrintString "Not Player" true true "(R=1.000000,G=0.000000,B=0.871570,A=1.000000)"))))

(event OnComponentBeginOverlap(entrada)
  (params (OverlappedComponent :type Primitive%20Component%20Object%20Reference) (OtherActor :type Actor%20Object%20Reference) (OtherComp :type Primitive%20Component%20Object%20Reference) (OtherBodyIndex :type Integer) (bFromSweep :type Boolean) (SweepResult :type Hit%20Result%20Structure%20%28by%20ref%29))
  (bind _westwalldoor (Variables|Default|GetWestWallDoor))
  (bind _relativelocation (Variables|/Script/Engine.SceneComponent|GetRelativeLocation _westwalldoor))
  (if (not (Variables|Default|GetplayerInside))
    (Variables|Default|SetplayerInside true)
    (Components|MoveComponentTo _westwalldoor (Math|Vector|MakeVector (.x _relativelocation) (.y _relativelocation) (+ (.z _relativelocation) 3e+02)) "0, 0, 0" false false 1.0 false)
    (Development|PrintString "Crida funció des del pare")
    (Variables|Default|SetspawnBoss true)))

(event OnComponentBeginOverlap(EndLevelColl)
  (params (OverlappedComponent :type Primitive%20Component%20Object%20Reference) (OtherActor :type Actor%20Object%20Reference) (OtherComp :type Primitive%20Component%20Object%20Reference) (OtherBodyIndex :type Integer) (bFromSweep :type Boolean) (SweepResult :type Hit%20Result%20Structure%20%28by%20ref%29))
  (bind _returnvalue (Game|Player|GetPlayerPawn 0))
  ;[1 1 1] Acabar Nivell
  (if (== OtherActor _returnvalue)
    (bind _asbp_character (Utilities|Casting|CastToBP_Character _returnvalue))
    (Default|SaveRunData _asbp_character false false)
    (Game|OpenLevel(byObjectReference) "/Game/Levels/EndRun.EndRun")
    (else
      (Development|PrintString "Not Player" true true "(R=1.000000,G=0.000000,B=0.871570,A=1.000000)"))))

(event OnComponentBeginOverlap(NewLevelColl)
  (params (OverlappedComponent :type Primitive%20Component%20Object%20Reference) (OtherActor :type Actor%20Object%20Reference) (OtherComp :type Primitive%20Component%20Object%20Reference) (OtherBodyIndex :type Integer) (bFromSweep :type Boolean) (SweepResult :type Hit%20Result%20Structure%20%28by%20ref%29))
  ;[1 1 1] Continuar
  (Development|PrintString "Colliison" true true "(R=1.000000,G=0.000000,B=0.871570,A=1.000000)")
  (if (== OtherActor (Game|Player|GetPlayerPawn 0))
    (bind _asbp_character (Utilities|Casting|CastToBP_Character (Game|Player|GetPlayerPawn 0)))
    (Default|SaveRunData _asbp_character true false)
    (bind _asmy_game_instance (Utilities|Casting|CastToMyGameInstance (Game|GetGameInstance)))
    (if (>= (Variables|/Game/SaveLoad/MyGameInstance.MyGameInstance_C|GetrunLoopNum _asmy_game_instance) 3)
      (Game|OpenLevel(byObjectReference) "/Game/Levels/EndRun.EndRun")
      (else
        (bind _returnvalue (UserInterface|CreateWidget "/Game/UI/LoadingScreen.LoadingScreen_C"))
        (bind _asmy_game_instance_2 (Utilities|Casting|CastToMyGameInstance (Game|GetGameInstance)))
        (Variables|/Game/SaveLoad/MyGameInstance.MyGameInstance_C|SettoBossRoom _asmy_game_instance_2 false)
        (UserInterface|Viewport|AddtoViewport _returnvalue 0)
        (Utilities|FlowControl|Delay 2.0)
        (Game|OpenLevel(byObjectReference) "/Game/Levels/LevelGenerator.LevelGenerator")))
    (else
      (Development|PrintString "Not Player" true true "(R=1.000000,G=0.000000,B=0.871570,A=1.000000)"))))

(fn ConstructionScript)

(fn PlayerEnters
  (Development|PrintString "In Boss Room" true true "(R=0.144696,G=0.734375,B=0.000000,A=1.000000)" 5.0))

(fn PlayerGoBack
  (Default|ChangeCamera (Variables|Default|GetrefCamManager) (Variables|Default|GetpreBossRoomX) (Variables|Default|GetpreBossRoomY)))

(fn PlaceNextLevelDoor
  (bind _nextleveldoor (Variables|Default|GetNextLevelDoor))
  (bind _returnvalue (Transformation|GetWorldLocation _nextleveldoor))
  (Transformation|SetWorldLocation _nextleveldoor (Math|Vector|MakeVector (.x _returnvalue) (.y _returnvalue) (+ (.z _returnvalue) 5.2e+02)) false false))

(fn EnemyBossSetup
  (params (_enemy :type Pawn%20Object%20Reference))
  (bind _aspersecutor (Utilities|Casting|CastToPersecutor _enemy)
    (:then
      (Variables|/Game/enemy/BaseEnemics.BaseEnemics_C|SetEnemyBossRoom _aspersecutor self))
    (:CastFailed
      (bind _asgorgona_petita_torreta (Utilities|Casting|CastToGorgonaPetitaTorreta _enemy)
        (:then
          (Variables|/Game/enemy/BaseEnemics.BaseEnemics_C|SetEnemyBossRoom _asgorgona_petita_torreta self))
        (:CastFailed
          (bind _asgran_gorgona_boss (Utilities|Casting|CastToGranGorgonaBoss _enemy)
            (:then
              (Variables|/Game/enemy/BaseEnemics.BaseEnemics_C|SetEnemyBossRoom _asgran_gorgona_boss self))
            (:CastFailed
              (bind _ascabeza_de_hydra_principal (Utilities|Casting|CastToCabeza_de_Hydra_principal _enemy)
                (:then
                  (Variables|/Game/enemy/BaseEnemics.BaseEnemics_C|SetEnemyBossRoom _ascabeza_de_hydra_principal self))
                (:CastFailed
                  (bind _ascabeza_de_hydra (Utilities|Casting|CastToCabeza_de_Hydra _enemy))
                  (Variables|/Game/enemy/BaseEnemics.BaseEnemics_C|SetEnemyBossRoom _ascabeza_de_hydra self)))))))))
  (Math|Integer|IncrementInt (Variables|Default|GetactualEnemies)))

(fn EnemyDead
  (Math|Integer|DecrementInt (Variables|Default|GetactualEnemies)))

(fn CheckAmountEnemies
  (if (<= (Variables|Default|GetactualEnemies) 0)
    (CallFunction|PlaceNextLevelDoor)))

(fn StopBossMusic
  (Utilities|FlowControl|DoOnce false
    (:Completed
      (Audio|Components|Audio|Stop (Variables|Default|GetBossBaseMusic))
      (Audio|Components|Audio|Stop (Variables|Default|GetBossLoopMusic)))))