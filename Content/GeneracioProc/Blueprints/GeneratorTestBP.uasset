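; Test procedural level generator that builds a grid of room actors for one of three island types on BeginPlay.
; Helper functions clear data, generate the layout and assign room IDs and special rooms, then nested loops visit each cell.
; Valid cells spawn a room class chosen by island type and ID at a spaced position, then receive their door configuration through ModifyDoors.
; Many IDs still spawn the placeholder BaseGeneralRoom.
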(event EventBeginPlay
  (Class|GeneratorV1|ClearData)
  (Class|GeneratorV1|GenerateLevel)
  (Class|GeneratorV1|SetRoomsID)
  (Class|GeneratorV1|SetSpecialRooms)
  ;[1 1 1 1 15] Loop pel la 2na Dimensió
  (for _index (range 0 (Variables|Default|GetmidaMapa))
    (Variables|Default|SetloopX _index)
    ;[1 1 1 1 15] Lopp per la 1ra Dimensió
    (for _index_2 (range 0 (Variables|Default|GetmidaMapa))
      (Variables|Default|SetloopY _index_2)
      ;[1 1 1 1 15] Si la sala té alguna dirreció i una ID vàlida
      (bind _returnvalue (Class|GeneratorV1|GetRoomID (Variables|Default|GetloopX) (Variables|Default|GetloopY)))
      (bind _output_get (Variables|Default|SetloopRoomID _returnvalue))
      (bind _returnvalue_2 (Class|GeneratorV1|GetNumDoors (Variables|Default|GetloopX) (Variables|Default|GetloopY)))
      (bind _output_get_2 (Variables|Default|SetloopDoorNum _returnvalue_2))
      (if (and (!= _output_get -1) (!= _output_get_2 -1))
        ;[1 1 1 1 15] Vector de la nova posició
        (bind _output_get_3 (Variables|Default|Set_spawnLocation (Math|Vector|MakeVector (Math|Conversions|ToFloat(Integer) (* (Variables|Default|GetdistanciaEnX) (Variables|Default|GetloopX))) (Math|Conversions|ToFloat(Integer) (* (Variables|Default|GetdistanciaEnY) (Variables|Default|GetloopY))) 0.0)))
        (Variables|Default|Set_spawnTransform (Math|Conversions|ToTransform(Vector) _output_get_3))
        (switch int (Variables|Default|Get_tipusIlla)
          (:Default
            (Development|PrintString "Num Tipus Illa Erroni" true true "(R=1.000000,G=0.000000,B=0.028557,A=1.000000)" 6e+01))
          (:0
            (switch int (Variables|Default|GetloopRoomID)
              (:Default
                (Development|PrintString "Room ID Erroni" true true "(R=1.000000,G=0.000000,B=0.028557,A=1.000000)" 6e+01))
              (:0
                (bind _returnvalue_3 (Game|SpawnActorfromClass "/Game/GeneracioProc/Blueprints/Grega/G_ClearRoomBP.G_ClearRoomBP_C" (Variables|Default|Get_spawnTransform) "AdjustIfPossibleButAlwaysSpawn" 0 0))
                (Default|ModifyDoors _returnvalue_3 (Variables|Default|GetloopDoorNum)))
              (:1
                (bind _returnvalue_4 (Game|SpawnActorfromClass "/Game/GeneracioProc/Blueprints/Grega/G_BossRoomBP.G_BossRoomBP_C" (Variables|Default|Get_spawnTransform) "AdjustIfPossibleButAlwaysSpawn" 0 0))
                (Default|ModifyDoors _returnvalue_4 (Variables|Default|GetloopDoorNum)))
              (:2
                (bind _returnvalue_5 (Game|SpawnActorfromClass "/Game/GeneracioProc/Blueprints/Grega/G_SpecialRoomBP.G_SpecialRoomBP_C" (Variables|Default|Get_spawnTransform) "AdjustIfPossibleButAlwaysSpawn" 0 0))
                (Default|ModifyDoors _returnvalue_5 (Variables|Default|GetloopDoorNum)))
              (:3
                (bind _returnvalue_6 (Game|SpawnActorfromClass "/Game/GeneracioProc/Blueprints/Grega/OtherRooms_G/G_Room1BP.G_Room1BP_C" (Variables|Default|Get_spawnTransform) "AdjustIfPossibleButAlwaysSpawn" 0 0))
                (Default|ModifyDoors _returnvalue_6 (Variables|Default|GetloopDoorNum)))
              (:4
                (bind _returnvalue_7 (Game|SpawnActorfromClass "/Game/GeneracioProc/Blueprints/Grega/OtherRooms_G/G_Room2BP.G_Room2BP_C" (Variables|Default|Get_spawnTransform) "AdjustIfPossibleButAlwaysSpawn" 0 0))
                (Default|ModifyDoors _returnvalue_7 (Variables|Default|GetloopDoorNum)))
              (:5
                (bind _returnvalue_8 (Game|SpawnActorfromClass "/Game/GeneracioProc/Blueprints/Grega/OtherRooms_G/G_Room3BP.G_Room3BP_C" (Variables|Default|Get_spawnTransform) "AdjustIfPossibleButAlwaysSpawn" 0 0))
                (Default|ModifyDoors _returnvalue_8 (Variables|Default|GetloopDoorNum)))
              (:6
                (bind _returnvalue_9 (Game|SpawnActorfromClass "/Game/GeneracioProc/Blueprints/Grega/OtherRooms_G/G_Room4BP.G_Room4BP_C" (Variables|Default|Get_spawnTransform) "AdjustIfPossibleButAlwaysSpawn" 0 0))
                (Default|ModifyDoors _returnvalue_9 (Variables|Default|GetloopDoorNum)))
              (:7
                (bind _returnvalue_10 (Game|SpawnActorfromClass "/Game/GeneracioProc/Blueprints/Grega/OtherRooms_G/G_Room5BP.G_Room5BP_C" (Variables|Default|Get_spawnTransform) "AdjustIfPossibleButAlwaysSpawn" 0 0))
                (Default|ModifyDoors _returnvalue_10 (Variables|Default|GetloopDoorNum)))
              (:8
                (bind _returnvalue_11 (Game|SpawnActorfromClass "/Game/GeneracioProc/Blueprints/Grega/OtherRooms_G/G_Room6BP.G_Room6BP_C" (Variables|Default|Get_spawnTransform) "AdjustIfPossibleButAlwaysSpawn" 0 0))
                (Default|ModifyDoors _returnvalue_11 (Variables|Default|GetloopDoorNum)))
              (:9
                (bind _returnvalue_12 (Game|SpawnActorfromClass "/Game/GeneracioProc/Blueprints/Grega/OtherRooms_G/G_Room7BP.G_Room7BP_C" (Variables|Default|Get_spawnTransform) "AdjustIfPossibleButAlwaysSpawn" 0 0))
                (Default|ModifyDoors _returnvalue_12 (Variables|Default|GetloopDoorNum)))
              (:10
                (bind _returnvalue_13 (Game|SpawnActorfromClass "/Game/GeneracioProc/Blueprints/BaseGeneralRoom.BaseGeneralRoom_C" (Variables|Default|Get_spawnTransform) "AdjustIfPossibleButAlwaysSpawn" 0 0))
                (Default|ModifyDoors _returnvalue_13 (Variables|Default|GetloopDoorNum)))
              (:11
                (bind _returnvalue_14 (Game|SpawnActorfromClass "/Game/GeneracioProc/Blueprints/BaseGeneralRoom.BaseGeneralRoom_C" (Variables|Default|Get_spawnTransform) "AdjustIfPossibleButAlwaysSpawn" 0 0))
                (Default|ModifyDoors _returnvalue_14 (Variables|Default|GetloopDoorNum)))
              (:12
                (bind _returnvalue_15 (Game|SpawnActorfromClass "/Game/GeneracioProc/Blueprints/BaseGeneralRoom.BaseGeneralRoom_C" (Variables|Default|Get_spawnTransform) "AdjustIfPossibleButAlwaysSpawn" 0 0))
                (Default|ModifyDoors _returnvalue_15 (Variables|Default|GetloopDoorNum)))
              (:13
                (bind _returnvalue_16 (Game|SpawnActorfromClass "/Game/GeneracioProc/Blueprints/BaseGeneralRoom.BaseGeneralRoom_C" (Variables|Default|Get_spawnTransform) "AdjustIfPossibleButAlwaysSpawn" 0 0))
                (Default|ModifyDoors _returnvalue_16 (Variables|Default|GetloopDoorNum)))
              (:14
                (bind _returnvalue_17 (Game|SpawnActorfromClass "/Game/GeneracioProc/Blueprints/BaseGeneralRoom.BaseGeneralRoom_C" (Variables|Default|Get_spawnTransform) "AdjustIfPossibleButAlwaysSpawn" 0 0))
                (Default|ModifyDoors _returnvalue_17 (Variables|Default|GetloopDoorNum)))
              (:15
                (bind _returnvalue_18 (Game|SpawnActorfromClass "/Game/GeneracioProc/Blueprints/BaseGeneralRoom.BaseGeneralRoom_C" (Variables|Default|Get_spawnTransform) "AdjustIfPossibleButAlwaysSpawn" 0 0))
                (Default|ModifyDoors _returnvalue_18 (Variables|Default|GetloopDoorNum)))
              (:16
                (bind _returnvalue_19 (Game|SpawnActorfromClass "/Game/GeneracioProc/Blueprints/BaseGeneralRoom.BaseGeneralRoom_C" (Variables|Default|Get_spawnTransform) "AdjustIfPossibleButAlwaysSpawn" 0 0))
                (Default|ModifyDoors _returnvalue_19 (Variables|Default|GetloopDoorNum)))
              (:17
                (bind _returnvalue_20 (Game|SpawnActorfromClass "/Game/GeneracioProc/Blueprints/BaseGeneralRoom.BaseGeneralRoom_C" (Variables|Default|Get_spawnTransform) "AdjustIfPossibleButAlwaysSpawn" 0 0))
                (Default|ModifyDoors _returnvalue_20 (Variables|Default|GetloopDoorNum)))
              (:18
                (bind _returnvalue_21 (Game|SpawnActorfromClass "/Game/GeneracioProc/Blueprints/BaseGeneralRoom.BaseGeneralRoom_C" (Variables|Default|Get_spawnTransform) "AdjustIfPossibleButAlwaysSpawn" 0 0))
                (Default|ModifyDoors _returnvalue_21 (Variables|Default|GetloopDoorNum)))
              (:19
                (bind _returnvalue_22 (Game|SpawnActorfromClass "/Game/GeneracioProc/Blueprints/BaseGeneralRoom.BaseGeneralRoom_C" (Variables|Default|Get_spawnTransform) "AdjustIfPossibleButAlwaysSpawn" 0 0))
                (Default|ModifyDoors _returnvalue_22 (Variables|Default|GetloopDoorNum)))
              (:20
                (bind _returnvalue_23 (Game|SpawnActorfromClass "/Game/GeneracioProc/Blueprints/BaseGeneralRoom.BaseGeneralRoom_C" (Variables|Default|Get_spawnTransform) "AdjustIfPossibleButAlwaysSpawn" 0 0))
                (Default|ModifyDoors _returnvalue_23 (Variables|Default|GetloopDoorNum)))
              (:21
                (bind _returnvalue_24 (Game|SpawnActorfromClass "/Game/GeneracioProc/Blueprints/BaseGeneralRoom.BaseGeneralRoom_C" (Variables|Default|Get_spawnTransform) "AdjustIfPossibleButAlwaysSpawn" 0 0))
                (Default|ModifyDoors _returnvalue_24 (Variables|Default|GetloopDoorNum)))
              (:22
                (bind _returnvalue_25 (Game|SpawnActorfromClass "/Game/GeneracioProc/Blueprints/BaseGeneralRoom.BaseGeneralRoom_C" (Variables|Default|Get_spawnTransform) "AdjustIfPossibleButAlwaysSpawn" 0 0))
                (Default|ModifyDoors _returnvalue_25 (Variables|Default|GetloopDoorNum)))))
          (:1
            (switch int (Variables|Default|GetloopRoomID)
              (:Default
                (Development|PrintString "Room ID Erroni" true true "(R=1.000000,G=0.000000,B=0.028557,A=1.000000)" 6e+01))
              (:0
                (bind _returnvalue_26 (Game|SpawnActorfromClass "/Game/GeneracioProc/Blueprints/Grega/G_ClearRoomBP.G_ClearRoomBP_C" (Variables|Default|Get_spawnTransform) "AdjustIfPossibleButAlwaysSpawn" 0 0))
                (Default|ModifyDoors _returnvalue_26 (Variables|Default|GetloopDoorNum)))
              (:1
                (bind _returnvalue_27 (Game|SpawnActorfromClass "/Game/GeneracioProc/Blueprints/Grega/G_BossRoomBP.G_BossRoomBP_C" (Variables|Default|Get_spawnTransform) "AdjustIfPossibleButAlwaysSpawn" 0 0))
                (Default|ModifyDoors _returnvalue_27 (Variables|Default|GetloopDoorNum)))
              (:2
                (bind _returnvalue_28 (Game|SpawnActorfromClass "/Game/GeneracioProc/Blueprints/Grega/G_SpecialRoomBP.G_SpecialRoomBP_C" (Variables|Default|Get_spawnTransform) "AdjustIfPossibleButAlwaysSpawn" 0 0))
                (Default|ModifyDoors _returnvalue_28 (Variables|Default|GetloopDoorNum)))
              (:3
                (bind _returnvalue_29 (Game|SpawnActorfromClass "/Game/GeneracioProc/Blueprints/BaseGeneralRoom.BaseGeneralRoom_C" (Variables|Default|Get_spawnTransform) "AdjustIfPossibleButAlwaysSpawn" 0 0))
                (Default|ModifyDoors _returnvalue_29 (Variables|Default|GetloopDoorNum)))))
          (:2
            (switch int (Variables|Default|GetloopRoomID)
              (:Default
                (Development|PrintString "Room ID Erroni" true true "(R=1.000000,G=0.000000,B=0.028557,A=1.000000)" 6e+01))
              (:0
                (bind _returnvalue_30 (Game|SpawnActorfromClass "/Game/GeneracioProc/Blueprints/Grega/G_ClearRoomBP.G_ClearRoomBP_C" (Variables|Default|Get_spawnTransform) "AdjustIfPossibleButAlwaysSpawn" 0 0))
                (Default|ModifyDoors _returnvalue_30 (Variables|Default|GetloopDoorNum)))
              (:1
                (bind _returnvalue_31 (Game|SpawnActorfromClass "/Game/GeneracioProc/Blueprints/Grega/G_BossRoomBP.G_BossRoomBP_C" (Variables|Default|Get_spawnTransform) "AdjustIfPossibleButAlwaysSpawn" 0 0))
                (Default|ModifyDoors _returnvalue_31 (Variables|Default|GetloopDoorNum)))
              (:2
                (bind _returnvalue_32 (Game|SpawnActorfromClass "/Game/GeneracioProc/Blueprints/Grega/G_SpecialRoomBP.G_SpecialRoomBP_C" (Variables|Default|Get_spawnTransform) "AdjustIfPossibleButAlwaysSpawn" 0 0))
                (Default|ModifyDoors _returnvalue_32 (Variables|Default|GetloopDoorNum)))
              (:3
                (bind _returnvalue_33 (Game|SpawnActorfromClass "/Game/GeneracioProc/Blueprints/BaseGeneralRoom.BaseGeneralRoom_C" (Variables|Default|Get_spawnTransform) "AdjustIfPossibleButAlwaysSpawn" 0 0))
                (Default|ModifyDoors _returnvalue_33 (Variables|Default|GetloopDoorNum))))))))))

(fn ConstructionScript)