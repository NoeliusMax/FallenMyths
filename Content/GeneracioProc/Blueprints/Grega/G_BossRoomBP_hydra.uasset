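; Boss room Blueprint for the Hydra fight, which spawns the main Hydra head and additional heads by phase.
; Tick watches SpawnBoss and, through a DoOnce, spawns the main head at SpawnBoss0 and passes it to EnemyBossSetup.
; CridaCaps takes a phase index and spawns a secondary head at one of three turret spawn points, with the same setup.
; An unconnected branch for moving the west wall door never runs.
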(event EventTick
  (params (DeltaSeconds :type Float%20%28single-precision%29))
  (if (Variables|Default|GetspawnBoss)
    (Utilities|FlowControl|DoOnce false
      (:Completed
        (bind _returnvalue (AI|SpawnAIFromClass "/Game/enemy/Cabeza_de_Hydra_principal.Cabeza_de_Hydra_principal_C" 0 (Transformation|GetWorldLocation (Variables|Default|GetspawnBoss_0)) "0, 0, 0" false 0))
        (CallFunction|EnemyBossSetup _returnvalue)
        (Utilities|Casting|CastToCabeza_de_Hydra _returnvalue)))))

(fn ConstructionScript
  (|CallParentFunction))

(fn CridaCaps
  (params (fase :type Integer))
  (switch int fase
    (:0
      (bind _returnvalue (AI|SpawnAIFromClass "/Game/enemy/Cabeza_de_Hydra.Cabeza_de_Hydra_C" 0 (Transformation|GetWorldLocation (Variables|Default|Getspawntorreta4)) "0, 0, 0" false 0))
      (CallFunction|EnemyBossSetup _returnvalue))
    (:1
      (bind _returnvalue_2 (AI|SpawnAIFromClass "/Game/enemy/Cabeza_de_Hydra.Cabeza_de_Hydra_C" 0 (Transformation|GetWorldLocation (Variables|Default|Getspawntorreta1)) "0, 0, 0" false 0))
      (CallFunction|EnemyBossSetup _returnvalue_2))
    (:2
      (bind _returnvalue_3 (AI|SpawnAIFromClass "/Game/enemy/Cabeza_de_Hydra.Cabeza_de_Hydra_C" 0 (Transformation|GetWorldLocation (Variables|Default|Getspawntorreta3)) "0, 0, 0" false 0))
      (CallFunction|EnemyBossSetup _returnvalue_3))))