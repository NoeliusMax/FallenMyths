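; Room Blueprint for procedural level generation that spawns a Persecutor AI enemy the first time the player enters.
; Its PlayerEnters override calls the parent, sets the Descoberta flag, spawns the pawn at the Spawn component and passes it to EnemySetup.
; Door modification and construction defer to the parent room class, and the EventGraph holds only unconnected leftovers of the spawn logic and a room-coordinate label.
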(fn ConstructionScript
  (|CallParentFunction))

(fn ModifyDoors
  (params (nDoors :type Integer))
  (|CallParentFunction nDoors))

(fn PlayerEnters
  (|CallParentFunction)
  (if (not (Variables|Default|Getdescoberta))
    (Variables|Default|Setdescoberta true)
    (bind _returnvalue (AI|SpawnAIFromClass "/Game/enemy/Persecutor.Persecutor_C" 0 (Transformation|GetWorldLocation (Variables|Default|GetSpawn)) "0, 0, 0" false 0))
    (CallFunction|EnemySetup _returnvalue)))