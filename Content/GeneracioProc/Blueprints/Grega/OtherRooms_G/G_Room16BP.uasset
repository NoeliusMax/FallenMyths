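; Room 16 variant for procedural level generation, a child room Blueprint with scattered leaves and a single enemy encounter.
; The construction script adds a collision-free instanced static mesh component and fills it with a jittered grid of randomly yawed instances.
; On first player entry it marks the room discovered, spawns a GorgonaPetitaTorreta at the Spawn point and runs EnemySetup.
; BeginPlay writes the room's grid coordinates to a text component; door handling defers to the parent.
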(event EventBeginPlay
  (Rendering|Components|TextRender|SetText (Variables|Default|GetText) (Utilities|Text|ToText(String) (Utilities|String|Append (Utilities|String|Append (Utilities|String|ToString(Integer) (Variables|Default|GetroomX)) ",") (Utilities|String|ToString(Integer) (Variables|Default|GetroomY))))))

(fn ConstructionScript
  (bind _distance (Variables|Default|GetDistance))
  (bind _distancernd (Variables|Default|GetDistanceRND))
  (bind _distance_2 (Variables|Default|GetDistance))
  (bind _distancernd_2 (Variables|Default|GetDistanceRND))
  (bind _rotationrnd (Variables|Default|GetRotationRND))
  (|CallParentFunction)
  (bind _returnvalue (AddComponent|AddInstancedStaticMeshComponent (Components|GetOwner (Variables|Default|GetLEAVES)) false))
  (Collision|SetCollisionEnabled _returnvalue "NoCollision")
  (for _index (range 0 (Variables|Default|GetSize))
    (for _index_2 (range 0 (Variables|Default|GetSize))
      (Components|InstancedStaticMesh|AddInstance _returnvalue (Math|Transform|MakeRelativeTransform (Math|Transform|MakeTransform (Math|Vector|MakeVector (+ (* _index_2 _distance) (* _distance (Math|Random|RandomFloatinRange (* _distancernd -1.0) _distancernd))) (+ (* _index _distance_2) (* _distance_2 (Math|Random|RandomFloatinRange (* _distancernd_2 -1.0) _distancernd_2))) 0.0) (Math|Rotator|MakeRotator 0.0 0.0 (Math|Random|RandomFloatinRange (* _rotationrnd -1.0) _rotationrnd)) (Math|Conversions|ToVector(Float) (+ (Math|Random|RandomFloatinRange (* 0.0 -1.0) 0.0) 1.0))) (Math|Transform|MakeTransform "700.000000,700.000000, 0" "0, 0, 0" "0.990000,0.800000,1"))))))

(fn ModifyDoors
  (params (nDoors :type Integer))
  (|CallParentFunction nDoors))

(fn PlayerEnters
  (|CallParentFunction)
  (if (not (Variables|Default|Getdescoberta))
    (Variables|Default|Setdescoberta true)
    (bind _returnvalue (AI|SpawnAIFromClass "/Game/enemy/GorgonaPetitaTorreta.GorgonaPetitaTorreta_C" 0 (Transformation|GetWorldLocation (Variables|Default|GetSpawn)) "0, 0, 0" false 0))
    (CallFunction|EnemySetup _returnvalue)))