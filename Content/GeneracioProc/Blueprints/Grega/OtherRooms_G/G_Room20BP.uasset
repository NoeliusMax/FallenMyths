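; G_Room20BP is a room Blueprint, apparently for procedural level generation, that spawns enemies when the player first enters.
; Its PlayerEnters override runs the parent logic, then uses the Descoberta flag to spawn only once.
; It spawns two Persecutor AI pawns at the Spawn and Spawn1 component locations and passes each to EnemySetup.
; Construction and ModifyDoors only defer to the parent.
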(event EventBeginPlay)

(event Collision|EventActorBeginOverlap
  (params (OtherActor :type Actor%20Object%20Reference)))

(event EventTick
  (params (DeltaSeconds :type Float%20%28single-precision%29)))

(fn ConstructionScript
  (|CallParentFunction))

(fn PlayerEnters
  (|CallParentFunction)
  (if (not (Variables|Default|Getdescoberta))
    (Variables|Default|Setdescoberta true)
    (bind _returnvalue (AI|SpawnAIFromClass "/Game/enemy/Persecutor.Persecutor_C" 0 (Transformation|GetWorldLocation (Variables|Default|GetSpawn)) "0, 0, 0" false 0))
    (CallFunction|EnemySetup _returnvalue)
    (bind _returnvalue_2 (AI|SpawnAIFromClass "/Game/enemy/Persecutor.Persecutor_C" 0 (Transformation|GetWorldLocation (Variables|Default|GetSpawn1)) "0, 0, 0" false 0))
    (CallFunction|EnemySetup _returnvalue_2)))

(fn ModifyDoors
  (params (nDoors :type Integer))
  (|CallParentFunction nDoors))