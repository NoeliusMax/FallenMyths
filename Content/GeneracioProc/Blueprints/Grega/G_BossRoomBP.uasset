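; Boss room Blueprint for the Grega set in procedural generation, which spawns a Gorgon boss encounter.
; Tick watches SpawnBoss and, through a DoOnce, spawns one GranGorgonaBoss and two GorgonaPetitaTorreta turrets at scene component locations.
; Each spawned enemy is passed to EnemyBossSetup, and construction defers to the parent class.
; A disconnected fragment for moving the west wall door never runs.
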(event EventTick
  (params (DeltaSeconds :type Float%20%28single-precision%29))
  (if (Variables|Default|GetspawnBoss)
    (Utilities|FlowControl|DoOnce false
      (:Completed
        (bind _returnvalue (Game|SpawnActorfromClass "/Game/enemy/GranGorgonaBoss.GranGorgonaBoss_C" (Math|Conversions|ToTransform(Vector) (Transformation|GetWorldLocation (Variables|Default|GetspawnBoss_0))) "Undefined" 0 0))
        (CallFunction|EnemyBossSetup _returnvalue)
        (bind _returnvalue_2 (Game|SpawnActorfromClass "/Game/enemy/GorgonaPetitaTorreta.GorgonaPetitaTorreta_C" (Math|Conversions|ToTransform(Vector) (Transformation|GetWorldLocation (Variables|Default|Getspawntorreta))) "Undefined" 0 0))
        (CallFunction|EnemyBossSetup _returnvalue_2)
        (bind _returnvalue_3 (Game|SpawnActorfromClass "/Game/enemy/GorgonaPetitaTorreta.GorgonaPetitaTorreta_C" (Math|Conversions|ToTransform(Vector) (Transformation|GetWorldLocation (Variables|Default|Getspawntorreta1))) "Undefined" 0 0))
        (CallFunction|EnemyBossSetup _returnvalue_3)))))

(fn ConstructionScript
  (|CallParentFunction))