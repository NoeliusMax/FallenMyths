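; Final room Blueprint for the procedurally generated levels, with exits to end or continue the run and a portal to the boss.
; Three overlap colliders act only on the player pawn: two open the EndRun or LevelGenerator level.
; The portal moves the character to BossPos and sets the view target to the owner of the player's camera.
; PlayerEnters is empty, and non-player overlaps only print debug text.
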(event OnComponentBeginOverlap(PlayerPortalCol)
  (params (OverlappedComponent :type Primitive%20Component%20Object%20Reference) (OtherActor :type Actor%20Object%20Reference) (OtherComp :type Primitive%20Component%20Object%20Reference) (OtherBodyIndex :type Integer) (bFromSweep :type Boolean) (SweepResult :type Hit%20Result%20Structure%20%28by%20ref%29))
  (bind _returnvalue (Game|Player|GetPlayerPawn 0))
  ;[1 1 1] Player TP to Boss
  (Development|PrintString "To Boss Room" true true "(R=1.000000,G=0.000000,B=0.871570,A=1.000000)")
  (if (== OtherActor _returnvalue)
    (bind _ascharacter (Utilities|Casting|CastToCharacter _returnvalue))
    (Transformation|SetActorLocation _ascharacter (Variables|Default|GetbossPos) false false)
    (bind _asbp_character (Utilities|Casting|CastToBP_Character _returnvalue))
    (Game|Player|SetViewTargetwithBlend (Game|GetPlayerController 0) (Components|GetOwner (Variables|/Game/Player/Assets/PaperZ/BP_Character.BP_Character_C|GetPlayerCamera _asbp_character)) 0.0 "VTBlend_Linear" 0.0 false)
    (else
      (Development|PrintString "Not Player" true true "(R=1.000000,G=0.000000,B=0.871570,A=1.000000)"))))

(event OnComponentBeginOverlap(EndLevelColl)
  (params (OverlappedComponent :type Primitive%20Component%20Object%20Reference) (OtherActor :type Actor%20Object%20Reference) (OtherComp :type Primitive%20Component%20Object%20Reference) (OtherBodyIndex :type Integer) (bFromSweep :type Boolean) (SweepResult :type Hit%20Result%20Structure%20%28by%20ref%29))
  ;[1 1 1] Acabar Nivell
  (if (== OtherActor (Game|Player|GetPlayerPawn 0))
    (Game|OpenLevel(byObjectReference) "/Game/Levels/EndRun.EndRun")
    (else
      (Development|PrintString "Not Player" true true "(R=1.000000,G=0.000000,B=0.871570,A=1.000000)"))))

(event OnComponentBeginOverlap(NewLevelColl)
  (params (OverlappedComponent :type Primitive%20Component%20Object%20Reference) (OtherActor :type Actor%20Object%20Reference) (OtherComp :type Primitive%20Component%20Object%20Reference) (OtherBodyIndex :type Integer) (bFromSweep :type Boolean) (SweepResult :type Hit%20Result%20Structure%20%28by%20ref%29))
  ;[1 1 1] Continuar
  (Development|PrintString "Colliison" true true "(R=1.000000,G=0.000000,B=0.871570,A=1.000000)")
  (if (== OtherActor (Game|Player|GetPlayerPawn 0))
    (Game|OpenLevel(byObjectReference) "/Game/Levels/LevelGenerator.LevelGenerator")
    (else
      (Development|PrintString "Not Player" true true "(R=1.000000,G=0.000000,B=0.871570,A=1.000000)"))))

(fn ConstructionScript
  (|CallParentFunction))

(fn PlayerEnters)