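; Clear room of a procedurally generated layout, with four-way doors that move the player between rooms.
; ModifyDoors decodes a 1–15 bitmask (north, south, east, west) to show open doors and disable colliders on other sides.
; BeginPlay teleports the player to StartCube.
; Door overlaps offset the player by ModPos (east hard-coded), call MoveCam and clear CanTP against retriggering; a comment flags east as repeatedly moving the player.
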(event OnComponentBeginOverlap(NorthCollider)
  (params (OverlappedComponent :type Primitive%20Component%20Object%20Reference) (OtherActor :type Actor%20Object%20Reference) (OtherComp :type Primitive%20Component%20Object%20Reference) (OtherBodyIndex :type Integer) (bFromSweep :type Boolean) (SweepResult :type Hit%20Result%20Structure%20%28by%20ref%29))
  (bind _returnvalue (Game|Player|GetPlayerPawn 0))
  (bind _returnvalue_2 (Transformation|GetActorLocation _returnvalue))
  ;[1 1 1] Nord
  (if (== OtherActor _returnvalue)
    (bind _asbp_character (Utilities|Casting|CastToBP_Character _returnvalue)
      (:then
        (if (Variables|/Game/Player/Assets/PaperZ/BP_Character.BP_Character_C|GetcanTP _asbp_character)
          (Development|PrintString "Nord Y -" true true "(R=1.000000,G=0.000000,B=0.028831,A=1.000000)" 5.0)
          (Transformation|SetActorLocation _returnvalue (Math|Vector|MakeVector (.x _returnvalue_2) (- (.y _returnvalue_2) (Variables|Default|GetmodPos)) (.z _returnvalue_2)) false false)
          (bind _asbp_character_2 (Utilities|Casting|CastToBP_Character _returnvalue))
          (Default|MoveCam _asbp_character_2 1)
          (Variables|/Game/Player/Assets/PaperZ/BP_Character.BP_Character_C|SetcanTP _asbp_character_2 false)))
      (:CastFailed
        (Development|PrintString "Not Cast" true true "(R=1.000000,G=0.000000,B=0.871570,A=1.000000)")))
    (else
      (Development|PrintString "Not Player" true true "(R=1.000000,G=0.000000,B=0.871570,A=1.000000)"))))

(event OnComponentBeginOverlap(SouthCollider)
  (params (OverlappedComponent :type Primitive%20Component%20Object%20Reference) (OtherActor :type Actor%20Object%20Reference) (OtherComp :type Primitive%20Component%20Object%20Reference) (OtherBodyIndex :type Integer) (bFromSweep :type Boolean) (SweepResult :type Hit%20Result%20Structure%20%28by%20ref%29))
  (bind _returnvalue (Game|Player|GetPlayerPawn 0))
  (bind _returnvalue_2 (Transformation|GetActorLocation _returnvalue))
  ;[1 1 1] Sud
  (if (== OtherActor _returnvalue)
    (bind _asbp_character (Utilities|Casting|CastToBP_Character _returnvalue)
      (:then
        (if (Variables|/Game/Player/Assets/PaperZ/BP_Character.BP_Character_C|GetcanTP _asbp_character)
          (Development|PrintString "Sud Y +" true true "(R=1.000000,G=0.000000,B=0.028831,A=1.000000)" 5.0)
          (Transformation|SetActorLocation _returnvalue (Math|Vector|MakeVector (.x _returnvalue_2) (+ (.y _returnvalue_2) (Variables|Default|GetmodPos)) (.z _returnvalue_2)) false false)
          (bind _asbp_character_2 (Utilities|Casting|CastToBP_Character _returnvalue))
          (Default|MoveCam _asbp_character_2 2)
          (Variables|/Game/Player/Assets/PaperZ/BP_Character.BP_Character_C|SetcanTP _asbp_character_2 false)))
      (:CastFailed
        (Development|PrintString "Not Cast" true true "(R=1.000000,G=0.000000,B=0.871570,A=1.000000)")))
    (else
      (Development|PrintString "Not Player" true true "(R=1.000000,G=0.000000,B=0.871570,A=1.000000)"))))

(event OnComponentBeginOverlap(EastCollider)
  (params (OverlappedComponent :type Primitive%20Component%20Object%20Reference) (OtherActor :type Actor%20Object%20Reference) (OtherComp :type Primitive%20Component%20Object%20Reference) (OtherBodyIndex :type Integer) (bFromSweep :type Boolean) (SweepResult :type Hit%20Result%20Structure%20%28by%20ref%29))
  (bind _returnvalue (Game|Player|GetPlayerPawn 0))
  (bind _returnvalue_2 (Transformation|GetActorLocation _returnvalue))
  ;[1 1 1] Est
  ;;[1 1 1 1 16] Aquesta zona no funciona, ens mou el jugador diverses vegades, muiltiples print string
  (if (== OtherActor _returnvalue)
    (bind _asbp_character (Utilities|Casting|CastToBP_Character _returnvalue)
      (:then
        (if (Variables|/Game/Player/Assets/PaperZ/BP_Character.BP_Character_C|GetcanTP _asbp_character)
          (Development|PrintString "Est X+" true true "(R=1.000000,G=0.000000,B=0.028831,A=1.000000)" 5.0)
          (Transformation|SetActorLocation _returnvalue (Math|Vector|MakeVector (+ (.x _returnvalue_2) 4e+02) (.y _returnvalue_2) (.z _returnvalue_2)) false true)
          (bind _asbp_character_2 (Utilities|Casting|CastToBP_Character _returnvalue))
          (Default|MoveCam _asbp_character_2 3)
          (Variables|/Game/Player/Assets/PaperZ/BP_Character.BP_Character_C|SetcanTP _asbp_character_2 false)))
      (:CastFailed
        (Development|PrintString "Not Cast" true true "(R=1.000000,G=0.000000,B=0.871570,A=1.000000)")))
    (else
      (Development|PrintString "Not Player" true true "(R=1.000000,G=0.000000,B=0.871570,A=1.000000)"))))

(event OnComponentBeginOverlap(WestCollider)
  (params (OverlappedComponent :type Primitive%20Component%20Object%20Reference) (OtherActor :type Actor%20Object%20Reference) (OtherComp :type Primitive%20Component%20Object%20Reference) (OtherBodyIndex :type Integer) (bFromSweep :type Boolean) (SweepResult :type Hit%20Result%20Structure%20%28by%20ref%29))
  (bind _returnvalue (Game|Player|GetPlayerPawn 0))
  (bind _returnvalue_2 (Transformation|GetActorLocation _returnvalue))
  ;[1 1 1] Oest
  (if (== OtherActor _returnvalue)
    (bind _asbp_character (Utilities|Casting|CastToBP_Character _returnvalue)
      (:then
        (if (Variables|/Game/Player/Assets/PaperZ/BP_Character.BP_Character_C|GetcanTP _asbp_character)
          (Development|PrintString "Oest X -" true true "(R=1.000000,G=0.000000,B=0.028831,A=1.000000)" 5.0)
          (Transformation|SetActorLocation _returnvalue (Math|Vector|MakeVector (- (.x _returnvalue_2) (Variables|Default|GetmodPos)) (.y _returnvalue_2) (.z _returnvalue_2)) false false)
          (bind _asbp_character_2 (Utilities|Casting|CastToBP_Character _returnvalue))
          (Default|MoveCam _asbp_character_2 4)
          (Variables|/Game/Player/Assets/PaperZ/BP_Character.BP_Character_C|SetcanTP _asbp_character_2 false)))
      (:CastFailed
        (Development|PrintString "Not Cast" true true "(R=1.000000,G=0.000000,B=0.871570,A=1.000000)")))
    (else
      (Development|PrintString "Not Player" true true "(R=1.000000,G=0.000000,B=0.871570,A=1.000000)"))))

(event EventBeginPlay
  ;[1 1 1] Per posar-hi el jugador al començar
  (bind _asbp_character (Utilities|Casting|CastToBP_Character (Game|Player|GetPlayerPawn 0)))
  (Default|Teleportto _asbp_character (Transformation|GetWorldLocation (Variables|Default|GetStartCube))))

(fn ConstructionScript)

(fn ModifyDoors
  (params (nDoors :type Integer))
  (bind _output_get (Variables|Default|Set_nDoors nDoors))
  (if (and (< _output_get 16) (> _output_get 0))
    (if (== (Variables|Default|Get_nDoors) 1)
      (Rendering|SetVisibility (Variables|Default|GetNorthDoor) true false)
      (Collision|SetCollisionEnabled (Variables|Default|GetSouthCollider) "NoCollision")
      (Collision|SetCollisionEnabled (Variables|Default|GetEastCollider) "NoCollision")
      (Collision|SetCollisionEnabled (Variables|Default|GetWestCollider) "NoCollision")
      (elif (== (Variables|Default|Get_nDoors) 2)
        (Rendering|SetVisibility (Variables|Default|GetSouthDoor) true false)
        (Collision|SetCollisionEnabled (Variables|Default|GetNorthCollider) "NoCollision")
        (Collision|SetCollisionEnabled (Variables|Default|GetEastCollider) "NoCollision")
        (Collision|SetCollisionEnabled (Variables|Default|GetWestCollider) "NoCollision")
        (elif (== (Variables|Default|Get_nDoors) 3)
          (Rendering|SetVisibility (Variables|Default|GetNorthDoor) true false)
          (Rendering|SetVisibility (Variables|Default|GetSouthDoor) true false)
          (Collision|SetCollisionEnabled (Variables|Default|GetEastCollider) "NoCollision")
          (Collision|SetCollisionEnabled (Variables|Default|GetWestCollider) "NoCollision")
          (elif (== (Variables|Default|Get_nDoors) 4)
            (Rendering|SetVisibility (Variables|Default|GetEastDoor) true false)
            (Collision|SetCollisionEnabled (Variables|Default|GetNorthCollider) "NoCollision")
            (Collision|SetCollisionEnabled (Variables|Default|GetSouthCollider) "NoCollision")
            (Collision|SetCollisionEnabled (Variables|Default|GetWestCollider) "NoCollision")
            (elif (== (Variables|Default|Get_nDoors) 5)
              (Rendering|SetVisibility (Variables|Default|GetNorthDoor) true false)
              (Rendering|SetVisibility (Variables|Default|GetEastDoor) true false)
              (Collision|SetCollisionEnabled (Variables|Default|GetSouthCollider) "NoCollision")
              (Collision|SetCollisionEnabled (Variables|Default|GetWestCollider) "NoCollision")
              (elif (== (Variables|Default|Get_nDoors) 6)
                (Rendering|SetVisibility (Variables|Default|GetEastDoor) true false)
                (Rendering|SetVisibility (Variables|Default|GetSouthDoor) true false)
                (Collision|SetCollisionEnabled (Variables|Default|GetNorthCollider) "NoCollision")
                (Collision|SetCollisionEnabled (Variables|Default|GetWestCollider) "NoCollision")
                (elif (== (Variables|Default|Get_nDoors) 7)
                  (Rendering|SetVisibility (Variables|Default|GetNorthDoor) true false)
                  (Rendering|SetVisibility (Variables|Default|GetEastDoor) true false)
                  (Rendering|SetVisibility (Variables|Default|GetSouthDoor) true false)
                  (Collision|SetCollisionEnabled (Variables|Default|GetWestCollider) "NoCollision")
                  (elif (== (Variables|Default|Get_nDoors) 8)
                    (Rendering|SetVisibility (Variables|Default|GetWestDoor) true false)
                    (Collision|SetCollisionEnabled (Variables|Default|GetNorthCollider) "NoCollision")
                    (Collision|SetCollisionEnabled (Variables|Default|GetSouthCollider) "NoCollision")
                    (Collision|SetCollisionEnabled (Variables|Default|GetEastCollider) "NoCollision")
                    (elif (== (Variables|Default|Get_nDoors) 9)
                      (Rendering|SetVisibility (Variables|Default|GetNorthDoor) true false)
                      (Rendering|SetVisibility (Variables|Default|GetWestDoor) true false)
                      (Collision|SetCollisionEnabled (Variables|Default|GetSouthCollider) "NoCollision")
                      (Collision|SetCollisionEnabled (Variables|Default|GetEastCollider) "NoCollision")
                      (elif (== (Variables|Default|Get_nDoors) 10)
                        (Rendering|SetVisibility (Variables|Default|GetWestDoor) true false)
                        (Rendering|SetVisibility (Variables|Default|GetSouthDoor) true false)
                        (Collision|SetCollisionEnabled (Variables|Default|GetNorthCollider) "NoCollision")
                        (Collision|SetCollisionEnabled (Variables|Default|GetEastCollider) "NoCollision")
                        (elif (== (Variables|Default|Get_nDoors) 11)
                          (Rendering|SetVisibility (Variables|Default|GetNorthDoor) true false)
                          (Rendering|SetVisibility (Variables|Default|GetWestDoor) true false)
                          (Rendering|SetVisibility (Variables|Default|GetSouthDoor) true false)
                          (Collision|SetCollisionEnabled (Variables|Default|GetEastCollider) "NoCollision")
                          (elif (== (Variables|Default|Get_nDoors) 12)
                            (Rendering|SetVisibility (Variables|Default|GetEastDoor) true false)
                            (Rendering|SetVisibility (Variables|Default|GetWestDoor) true false)
                            (Collision|SetCollisionEnabled (Variables|Default|GetNorthCollider) "NoCollision")
                            (Collision|SetCollisionEnabled (Variables|Default|GetSouthCollider) "NoCollision")
                            (elif (== (Variables|Default|Get_nDoors) 13)
                              (Rendering|SetVisibility (Variables|Default|GetNorthDoor) true false)
                              (Rendering|SetVisibility (Variables|Default|GetEastDoor) true false)
                              (Rendering|SetVisibility (Variables|Default|GetWestDoor) true false)
                              (Collision|SetCollisionEnabled (Variables|Default|GetSouthCollider) "NoCollision")
                              (elif (== (Variables|Default|Get_nDoors) 14)
                                (Rendering|SetVisibility (Variables|Default|GetSouthDoor) true false)
                                (Rendering|SetVisibility (Variables|Default|GetEastDoor) true false)
                                (Rendering|SetVisibility (Variables|Default|GetWestDoor) true false)
                                (Collision|SetCollisionEnabled (Variables|Default|GetNorthCollider) "NoCollision")
                                (elif (== (Variables|Default|Get_nDoors) 15)
                                  (Rendering|SetVisibility (Variables|Default|GetNorthDoor) true false)
                                  (Rendering|SetVisibility (Variables|Default|GetSouthDoor) true false)
                                  (Rendering|SetVisibility (Variables|Default|GetEastDoor) true false)
                                  (Rendering|SetVisibility (Variables|Default|GetWestDoor) true false))))))))))))))))))