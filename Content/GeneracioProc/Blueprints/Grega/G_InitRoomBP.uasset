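; Starting room Blueprint for procedural generation that teleports the player to its StartCube on BeginPlay and flags itself as discovered (Descoberta).
; The construction script runs the parent's, then scatters non-colliding instances, apparently leaves, through a runtime-added InstancedStaticMesh component.
; Instances follow a Size-driven grid with random position, yaw and scale jitter, expressed relative to a hardcoded offset and scale.
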(event EventBeginPlay
  ;[1 1 1] Per posar-hi el jugador al començar
  (bind _asbp_character (Utilities|Casting|CastToBP_Character (Game|Player|GetPlayerPawn 0)))
  (Default|Teleportto _asbp_character (Transformation|GetWorldLocation (Variables|Default|GetStartCube)))
  (Variables|Default|Setdescoberta true))

(fn ConstructionScript
  (bind _distance (Variables|Default|GetDistance))
  (bind _distancernd (Variables|Default|GetDistanceRND))
  (bind _distance_2 (Variables|Default|GetDistance))
  (bind _distancernd_2 (Variables|Default|GetDistanceRND))
  (bind _rotationrnd (Variables|Default|GetRotationRND))
  (bind _scalernd (Variables|Default|GetScaleRND))
  (|CallParentFunction)
  (bind _returnvalue (AddComponent|AddInstancedStaticMeshComponent (Components|GetOwner (Variables|Default|GetLEAVES)) false))
  (Collision|SetCollisionEnabled _returnvalue "NoCollision")
  (for _index (range 0 (Variables|Default|GetSize))
    (for _index_2 (range 0 (Variables|Default|GetSize))
      (Components|InstancedStaticMesh|AddInstance _returnvalue (Math|Transform|MakeRelativeTransform (Math|Transform|MakeTransform (Math|Vector|MakeVector (+ (* _index_2 _distance) (* _distance (Math|Random|RandomFloatinRange (* _distancernd -1.0) _distancernd))) (+ (* _index _distance_2) (* _distance_2 (Math|Random|RandomFloatinRange (* _distancernd_2 -1.0) _distancernd_2))) 0.0) (Math|Rotator|MakeRotator 0.0 0.0 (Math|Random|RandomFloatinRange (* _rotationrnd -1.0) _rotationrnd)) (Math|Conversions|ToVector(Float) (+ (Math|Random|RandomFloatinRange (* _scalernd -1.0) _scalernd) 1.0))) (Math|Transform|MakeTransform "700.000000,700.000000, 0" "0, 0, 0" "0.990000,0.800000,1"))))))